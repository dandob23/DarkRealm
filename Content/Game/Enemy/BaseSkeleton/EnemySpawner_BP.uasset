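; Enemy spawner that creates random enemies inside a box zone, pausing while the player is inside its shut-off zone.
; SpawnCheck repeats on a delay, pruning invalid enemies and spawning until EnemyAmount is reached, where the loop stops rescheduling.
; A downward trace grounds each new enemy before randomizing its gear and items.
; The construction script applies configurable sizes to both zones and positions the shut-off zone.
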(event OnComponentBeginOverlap(ShutOffZone)
  (params (OverlappedComponent :type Primitive%20Component%20Object%20Reference) (OtherActor :type Actor%20Object%20Reference) (OtherComp :type Primitive%20Component%20Object%20Reference) (OtherBodyIndex :type Integer) (bFromSweep :type Boolean) (SweepResult :type Hit%20Result%20Structure%20%28by%20ref%29))
  (if (Actor|ActorHasTag OtherActor "Player")
    (Variables|Default|SetIsActorActive false)))

(event OnComponentEndOverlap(ShutOffZone)
  (params (OverlappedComponent :type Primitive%20Component%20Object%20Reference) (OtherActor :type Actor%20Object%20Reference) (OtherComp :type Primitive%20Component%20Object%20Reference) (OtherBodyIndex :type Integer))
  (if (Actor|ActorHasTag OtherActor "Player")
    (Variables|Default|SetIsActorActive true)))

(event Custom|SpawnCheck
  (bind _spawnzone (Variables|Default|GetSpawnZone))
  (bind _spawnedenemies (Variables|Default|GetSpawnedEnemies))
  (if (Variables|Default|GetIsActorActive)
    (for _array_element _spawnedenemies
      (Utilities|IsValid _array_element
        (:Is%20Not%20Valid
          (Utilities|Array|RemoveItem _spawnedenemies _array_element))))
    (if (not (>= (Utilities|Array|Length _spawnedenemies) (Variables|Default|GetEnemyAmount)))
      (bind _returnvalue (Game|SpawnActorfromClass (.OutItem (Utilities|Array|Random (Variables|Default|GetEnemiesToSpawn))) (Math|Transform|MakeTransform (Math|Random|RandomPointinBoundingBox (Transformation|GetWorldLocation _spawnzone) (Components|Box|GetScaledBoxExtent _spawnzone)) (Math|Rotator|MakeRotator 0.0 0.0 (Math|Random|RandomFloatinRange -1.8e+02 1.8e+02)) "1.000000,1.000000,1.000000") "Undefined" "MultiplyWithRoot" 0 0))
      (Utilities|IsValid _returnvalue
        (:Is%20Valid
          (Utilities|Array|AddUnique (Variables|Default|GetSpawnedEnemies) _returnvalue)
          (bind _output_get (Variables|Default|SetSpawnedUnitRef _returnvalue))
          (bind (_outhit _returnvalue_2) (Collision|LineTraceByChannel (Transformation|GetActorLocation _returnvalue) (- (Transformation|GetActorLocation _returnvalue) "0.000000,0.000000,10000.000000") "TraceTypeQuery1" false (Utilities|Array|MakeArray _output_get) "ForDuration"))
          (if _returnvalue_2
            (Transformation|SetActorLocation (Variables|Default|GetSpawnedUnitRef) (+ (.Location (Collision|BreakHitResult _outhit)) "0.000000,0.000000,90.000000") false false)
            (Default|RandomizeGearFunc (Variables|Default|GetSpawnedUnitRef))
            (Default|RandomizeItemFunc (Variables|Default|GetSpawnedUnitRef))))
        (:Is%20Not%20Valid
          _))
      (Utilities|FlowControl|Delay (Variables|Default|GetSpawnDelay) :!label _label)
      (CallFunction|SpawnCheck))
    (else
      (goto _label))))

(event EventBeginPlay
  (bind _spawnzone (Variables|Default|GetSpawnZone))
  (bind _spawnedenemies (Variables|Default|GetSpawnedEnemies))
  (if (Variables|Default|GetIsActorActive)
    (for _array_element _spawnedenemies
      (Utilities|IsValid _array_element
        (:Is%20Not%20Valid
          (Utilities|Array|RemoveItem _spawnedenemies _array_element))))
    (if (not (>= (Utilities|Array|Length _spawnedenemies) (Variables|Default|GetEnemyAmount)))
      (bind _returnvalue (Game|SpawnActorfromClass (.OutItem (Utilities|Array|Random (Variables|Default|GetEnemiesToSpawn))) (Math|Transform|MakeTransform (Math|Random|RandomPointinBoundingBox (Transformation|GetWorldLocation _spawnzone) (Components|Box|GetScaledBoxExtent _spawnzone)) (Math|Rotator|MakeRotator 0.0 0.0 (Math|Random|RandomFloatinRange -1.8e+02 1.8e+02)) "1.000000,1.000000,1.000000") "Undefined" "MultiplyWithRoot" 0 0))
      (Utilities|IsValid _returnvalue
        (:Is%20Valid
          (Utilities|Array|AddUnique (Variables|Default|GetSpawnedEnemies) _returnvalue)
          (bind _output_get (Variables|Default|SetSpawnedUnitRef _returnvalue))
          (bind (_outhit _returnvalue_2) (Collision|LineTraceByChannel (Transformation|GetActorLocation _returnvalue) (- (Transformation|GetActorLocation _returnvalue) "0.000000,0.000000,10000.000000") "TraceTypeQuery1" false (Utilities|Array|MakeArray _output_get) "ForDuration"))
          (if _returnvalue_2
            (Transformation|SetActorLocation (Variables|Default|GetSpawnedUnitRef) (+ (.Location (Collision|BreakHitResult _outhit)) "0.000000,0.000000,90.000000") false false)
            (Default|RandomizeGearFunc (Variables|Default|GetSpawnedUnitRef))
            (Default|RandomizeItemFunc (Variables|Default|GetSpawnedUnitRef))))
        (:Is%20Not%20Valid
          _))
      (Utilities|FlowControl|Delay (Variables|Default|GetSpawnDelay) :!label _label)
      (CallFunction|SpawnCheck))
    (else
      (goto _label))))

(fn ConstructionScript
  (bind _shutoffzone (Variables|Default|GetShutOffZone))
  (Components|Box|SetBoxExtent (Variables|Default|GetSpawnZone) (Variables|Default|GetSpawnZoneSize) true)
  (Components|Box|SetBoxExtent _shutoffzone (Variables|Default|GetShutOffZoneSize) true)
  (Transformation|SetRelativeLocation _shutoffzone (Variables|Default|GetShutOffZoneLocation) false false))