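; Base skeleton enemy AI that roams, spots the player, chases and attacks, then dies with a dust effect.
; A behaviour-mode switch re-enters itself to move between roam, see, investigate, chase and death states via AIMoveTo and the nearest patrol point.
; Chasing and attacking drain stamina, and exhaustion drops it into investigate to recover.
; PawnSensing adds a HUD enemy-list widget, and a montage notify triggers a damaging sphere trace.
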(event OnSeePawn(PawnSensing)
  (params (Pawn :type Pawn%20Object%20Reference))
  (bind _self self)
  (bind _playerref (Variables|Default|GetPlayerRef))
  ;[1 1 1] On Player character seen
  (if (not (Variables|Default|GetIsAiDead))
    (Utilities|FlowControl|DoOnce false
      (:Completed
        (Utilities|Array|AddUnique (Variables|/Game/Game/FirstPerson/Blueprints/BP_PLAYERCharacter.BP_PLAYERCharacter_C|GetEnemyList (Variables|Default|GetPlayerRef)) _self)
        (bind _returnvalue (UserInterface|CreateWidget "/Game/Game/UI/EnemyList_W.EnemyList_W_C" 0 _self))
        (Variables|Default|SetEnemyUiRef _returnvalue)
        (Widget|Panel|AddChild (Variables|/Game/Game/UI/W_StaticPlayerHUD.W_StaticPlayerHUD_C|GetEnemyList (Variables|/Game/Game/FirstPerson/Blueprints/BP_PLAYERCharacter.BP_PLAYERCharacter_C|GetStaticHudRef _playerref)) _returnvalue)
        (Variables|Default|SetAttackTarget _playerref)
        (Variables|Default|SetBehaviourMode "NewEnumerator4")
        (CallFunction|BehaviourUnit)))))

(event Custom|BehaviourUnit
  (bind _self self)
  (bind _charactermovement (Variables|Character|GetCharacterMovement))
  (bind _mesh (Variables|Character|GetMesh))
  (bind _charactermovement_2 (Variables|Character|GetCharacterMovement))
  (bind _charactermovement_3 (Variables|Character|GetCharacterMovement))
  (bind _attributecomponent_enemy (Variables|Default|GetAttributeComponent_ENEMY))
  (bind _attributecomponent_enemy_2 (Variables|Default|GetAttributeComponent_ENEMY))
  (bind _attributecomponent_enemy_3 (Variables|Default|GetAttributeComponent_ENEMY))
  (bind _returnvalue (Transformation|GetWorldTransform _mesh))
  (bind _maxstamina (Variables|/Game/Game/Enemy/BaseSkeleton/AttributeComponent_ENEMY.AttributeComponent_ENEMY_C|GetMaxStamina _attributecomponent_enemy_3))
  ;[1 1 1] Behaviour unit switch
  (switch Utilities|FlowControl|Switch|SwitchonBehaviourModes_ENUM (Variables|Default|GetBehaviourMode)
    (:NewEnumerator0
      ;[1 1 1] ROAM 1 STATE
      (AI|AIMoveTo self (.RandomLocation (AI|Navigation|GetRandomReachablePointinRadius (Transformation|GetActorLocation) (Variables|Default|GetRoamRadius) 0 0)) 0 5.0 true
        (:OnSuccess
          (CallFunction|UpdatePatrolPoint)
          (Utilities|FlowControl|Delay (Math|Random|RandomFloatinRange (Variables|Default|GetMinWaitTime) (Variables|Default|GetMaxWaitTime)))
          (if (Utilities|Enum|Equal(Enum) (Variables|Default|GetBehaviourMode) "NewEnumerator2")
            (CallFunction|ChasePlayer :!label _label)
            (else
              (Variables|Default|SetBehaviourMode "NewEnumerator1")
              (CallFunction|BehaviourUnit))))))
    (:NewEnumerator1
      ;[1 1 1] ROAM 2 STATE
      (AI|AIMoveTo self "0, 0, 0" (Variables|Default|GetPatrolPointRef) 5.0 true
        (:OnSuccess
          (Utilities|FlowControl|Delay (Math|Random|RandomFloatinRange (Variables|Default|GetMinWaitTime) (Variables|Default|GetMaxWaitTime)))
          (if (Utilities|Enum|Equal(Enum) (Variables|Default|GetBehaviourMode) "NewEnumerator2")
            (goto _label)
            (else
              (Variables|Default|SetBehaviourMode "NewEnumerator0")
              (CallFunction|BehaviourUnit))))))
    (:NewEnumerator4
      ;[1 1 1] SEE CHARACTER STATE
      (Components|Movement|StopMovementImmediately _charactermovement)
      (Variables|/Script/Engine.CharacterMovementComponent|SetMaxWalkSpeed _charactermovement 0.0)
      (Development|PrintString "Sees Player")
      (Utilities|FlowControl|Delay 1.0)
      (Variables|/Script/Engine.CharacterMovementComponent|SetMaxWalkSpeed _charactermovement 2e+02)
      (Variables|Default|SetBehaviourMode "NewEnumerator5")
      (CallFunction|BehaviourUnit))
    (:NewEnumerator5
      ;[1 1 1] INVESTIGATE PLAYER STATE
      (if (Variables|Default|GetIsAiDead)
        (Variables|Default|SetBehaviourMode "NewEnumerator6")
        (CallFunction|BehaviourUnit :!label _label_2)
        (else
          (if (Variables|Default|GetIsAiExhausted)
            (Variables|/Game/Game/Enemy/BaseSkeleton/AttributeComponent_ENEMY.AttributeComponent_ENEMY_C|SetStamina (Variables|Default|GetAttributeComponent_ENEMY) 0.0)
            (else
              (AI|AIMoveTo self "0, 0, 0" (Variables|Default|GetAttackTarget) (* (Variables|Default|GetMoveToPlayerAcceptanceRadius) 3.0) true
                (:OnSuccess
                  _))))
          (AI|AIMoveTo _self "0.000000,50.000000,0.000000" 0 5.0 true
            (:then
              _)
            (:OnSuccess
              (AI|AIMoveTo _self "0.000000,-100.000000,0.000000" 0 5.0 true
                (:then
                  _)
                (:OnSuccess
                  (AI|AIMoveTo _self "0.000000,50.000000,0.000000" 0 5.0 true
                    (:then
                      _)
                    (:OnSuccess
                      _))))))
          (if (Variables|Default|GetIsAiExhausted)
            (bind _output_get (Variables|/Game/Game/Enemy/BaseSkeleton/AttributeComponent_ENEMY.AttributeComponent_ENEMY_C|SetStamina _attributecomponent_enemy_3 (+ (Variables|/Game/Game/Enemy/BaseSkeleton/AttributeComponent_ENEMY.AttributeComponent_ENEMY_C|GetStamina _attributecomponent_enemy_3) 1e+01)))
            (Development|PrintString (Utilities|String|ToString(Float) _output_get) true true "(R=0.621116,G=0.000000,B=1.000000,A=1.000000)" 5.0)
            (Utilities|FlowControl|Delay 1.0)
            (if (>= (Variables|/Game/Game/Enemy/BaseSkeleton/AttributeComponent_ENEMY.AttributeComponent_ENEMY_C|GetStamina _attributecomponent_enemy_3) _maxstamina)
              (Variables|/Game/Game/Enemy/BaseSkeleton/AttributeComponent_ENEMY.AttributeComponent_ENEMY_C|SetStamina _attributecomponent_enemy_3 _maxstamina)
              (Variables|Default|SetIsAiExhausted false)
              (Variables|Default|SetBehaviourMode "NewEnumerator2")
              (CallFunction|BehaviourUnit))
            (else
              (Variables|Default|SetBehaviourMode "NewEnumerator2")
              (goto _label_2))))))
    (:NewEnumerator2
      ;[1 1 1] CHASE PLAYER STATE
      (if (Variables|Default|GetIsAiDead)
        (Variables|Default|SetBehaviourMode "NewEnumerator6")
        (CallFunction|BehaviourUnit :!label _label_3)
        (elif (Variables|Default|GetIsAiExhausted)
          (Variables|Default|SetBehaviourMode "NewEnumerator5")
          (CallFunction|BehaviourUnit)
          (else
            (Variables|/Script/Engine.CharacterMovementComponent|SetMaxWalkSpeed (Variables|Character|GetCharacterMovement) 4e+02)
            (AI|AIMoveTo self "0, 0, 0" (Variables|Default|GetAttackTarget) (Variables|Default|GetMoveToPlayerAcceptanceRadius) true
              (:then
                (bind _output_get_2 (Variables|/Game/Game/Enemy/BaseSkeleton/AttributeComponent_ENEMY.AttributeComponent_ENEMY_C|SetStamina _attributecomponent_enemy_2 (- (Variables|/Game/Game/Enemy/BaseSkeleton/AttributeComponent_ENEMY.AttributeComponent_ENEMY_C|GetStamina _attributecomponent_enemy_2) 5.0) :!label _label_4))
                (Development|PrintString (Utilities|String|ToString(Float) _output_get_2) true true "(R=1.000000,G=0.057921,B=0.000000,A=1.000000)" 5.0)
                (if (<= (Variables|/Game/Game/Enemy/BaseSkeleton/AttributeComponent_ENEMY.AttributeComponent_ENEMY_C|GetStamina _attributecomponent_enemy_2) 0.0)
                  (Variables|Default|SetIsAiExhausted true)
                  (else
                    (Variables|Default|SetIsAiExhausted false)))
                (if (Variables|Default|GetIsAiExhausted) :!label _label_5
                  (Variables|Default|SetBehaviourMode "NewEnumerator5")
                  (CallFunction|BehaviourUnit)
                  (else
                    (Utilities|FlowControl|Delay 0.2)
                    (goto _label_4))))
              (:OnSuccess
                (Utilities|FlowControl|DoOnce false
                  (:Completed
                    (Variables|Default|SetIsAiAttackingPlayer true)
                    (bind _notifyname (Animation|Montage|PlayMontage (Variables|Character|GetMesh) (Variables|Default|GetAttackMontage))
                      (:then
                        (Components|Movement|StopMovementImmediately _charactermovement_2)
                        (Variables|/Script/Engine.CharacterMovementComponent|SetMaxWalkSpeed _charactermovement_2 0.0)
                        (CallFunction|TrackPlayer)
                        (Utilities|FlowControl|DoOnce false
                          (:Completed
                            (bind _output_get_3 (Variables|/Game/Game/Enemy/BaseSkeleton/AttributeComponent_ENEMY.AttributeComponent_ENEMY_C|SetStamina _attributecomponent_enemy (- (Variables|/Game/Game/Enemy/BaseSkeleton/AttributeComponent_ENEMY.AttributeComponent_ENEMY_C|GetStamina _attributecomponent_enemy) 1e+01)))
                            (Development|PrintString (Utilities|String|ToString(Float) _output_get_3)))))
                      (:OnCompleted
                        (Utilities|FlowControl|Delay (Math|Random|RandomFloatinRange 0.1 0.3))
                        (Variables|Default|SetIsAiAttackingPlayer false)
                        (if (Variables|Default|GetIsAiDead)
                          (Variables|Default|SetBehaviourMode "NewEnumerator6")
                          (goto _label_3)
                          (else
                            (CallFunction|ReleaseAttack)
                            (Variables|/Script/Engine.CharacterMovementComponent|SetMaxWalkSpeed (Variables|Character|GetCharacterMovement) 4e+02)
                            (goto _label_3))))
                      (:OnNotifyBegin
                        (switch name _notifyname
                          (:AttackTrace
                            (CallFunction|AttackTrace))))))))
              (:OnFail
                (goto _label_5)))))))
    (:NewEnumerator6
      ;[1 1 1] DEATH STATE
      (Class|PanelWidget|RemoveChild (Variables|/Game/Game/UI/W_StaticPlayerHUD.W_StaticPlayerHUD_C|GetEnemyList (Variables|/Game/Game/FirstPerson/Blueprints/BP_PLAYERCharacter.BP_PLAYERCharacter_C|GetStaticHudRef (Variables|Default|GetPlayerRef))) (Variables|Default|GetEnemyUiRef))
      (Components|Movement|StopMovementImmediately _charactermovement_3)
      (Variables|/Script/Engine.CharacterMovementComponent|SetMaxWalkSpeed _charactermovement_3 0.0)
      (Components|Animation|PlayAnimation _mesh "/Game/Game/Enemy/Zombie_Death.Zombie_Death" false)
      (Utilities|FlowControl|Delay 5.0)
      (Effects|SpawnEmitteratLocation "/Game/InfinityBladeEffects/Effects/FX_Monsters/FX_Monster_SpiderBoss/Impact/P_SpiderChargeDust.P_SpiderChargeDust" (Math|Vector|MakeVector (.x (.location _returnvalue)) (.y (.location _returnvalue)) (- (.z (.location _returnvalue)) 5e+01)) (.rotation _returnvalue))
      (Actor|DestroyActor))))

(event Custom|ChasePlayer
  (bind _charactermovement (Variables|Character|GetCharacterMovement))
  (bind _attributecomponent_enemy (Variables|Default|GetAttributeComponent_ENEMY))
  (bind _attributecomponent_enemy_2 (Variables|Default|GetAttributeComponent_ENEMY))
  ;[1 1 1] CHASE PLAYER STATE
  (if (<= (Variables|/Game/Game/Enemy/BaseSkeleton/AttributeComponent_ENEMY.AttributeComponent_ENEMY_C|GetStamina (Variables|Default|GetAttributeComponent_ENEMY)) 0.0)
    (Variables|Default|SetIsAiExhausted true)
    (else
      (Variables|Default|SetIsAiExhausted false)))
  (if (Variables|Default|GetIsAiDead)
    (Variables|Default|SetBehaviourMode "NewEnumerator6")
    (CallFunction|BehaviourUnit :!label _label)
    (elif (Variables|Default|GetIsAiExhausted)
      (Variables|Default|SetBehaviourMode "NewEnumerator5")
      (CallFunction|BehaviourUnit)
      (else
        (Variables|/Script/Engine.CharacterMovementComponent|SetMaxWalkSpeed (Variables|Character|GetCharacterMovement) 4e+02)
        (AI|AIMoveTo self "0, 0, 0" (Variables|Default|GetAttackTarget) (Variables|Default|GetMoveToPlayerAcceptanceRadius) true
          (:then
            (bind _output_get (Variables|/Game/Game/Enemy/BaseSkeleton/AttributeComponent_ENEMY.AttributeComponent_ENEMY_C|SetStamina _attributecomponent_enemy_2 (- (Variables|/Game/Game/Enemy/BaseSkeleton/AttributeComponent_ENEMY.AttributeComponent_ENEMY_C|GetStamina _attributecomponent_enemy_2) 5.0) :!label _label_2))
            (Development|PrintString (Utilities|String|ToString(Float) _output_get) true true "(R=1.000000,G=0.057921,B=0.000000,A=1.000000)" 5.0)
            (if (<= (Variables|/Game/Game/Enemy/BaseSkeleton/AttributeComponent_ENEMY.AttributeComponent_ENEMY_C|GetStamina _attributecomponent_enemy_2) 0.0)
              (Variables|Default|SetIsAiExhausted true)
              (else
                (Variables|Default|SetIsAiExhausted false)))
            (if (Variables|Default|GetIsAiExhausted) :!label _label_3
              (Variables|Default|SetBehaviourMode "NewEnumerator5")
              (CallFunction|BehaviourUnit)
              (else
                (Utilities|FlowControl|Delay 0.2)
                (goto _label_2))))
          (:OnSuccess
            (Utilities|FlowControl|DoOnce false
              (:Completed
                (Variables|Default|SetIsAiAttackingPlayer true)
                (bind _notifyname (Animation|Montage|PlayMontage (Variables|Character|GetMesh) (Variables|Default|GetAttackMontage))
                  (:then
                    (Components|Movement|StopMovementImmediately _charactermovement)
                    (Variables|/Script/Engine.CharacterMovementComponent|SetMaxWalkSpeed _charactermovement 0.0)
                    (CallFunction|TrackPlayer)
                    (Utilities|FlowControl|DoOnce false
                      (:Completed
                        (bind _output_get_2 (Variables|/Game/Game/Enemy/BaseSkeleton/AttributeComponent_ENEMY.AttributeComponent_ENEMY_C|SetStamina _attributecomponent_enemy (- (Variables|/Game/Game/Enemy/BaseSkeleton/AttributeComponent_ENEMY.AttributeComponent_ENEMY_C|GetStamina _attributecomponent_enemy) 1e+01)))
                        (Development|PrintString (Utilities|String|ToString(Float) _output_get_2)))))
                  (:OnCompleted
                    (Utilities|FlowControl|Delay (Math|Random|RandomFloatinRange 0.1 0.3))
                    (Variables|Default|SetIsAiAttackingPlayer false)
                    (if (Variables|Default|GetIsAiDead)
                      (Variables|Default|SetBehaviourMode "NewEnumerator6")
                      (goto _label)
                      (else
                        (CallFunction|ReleaseAttack)
                        (Variables|/Script/Engine.CharacterMovementComponent|SetMaxWalkSpeed (Variables|Character|GetCharacterMovement) 4e+02)
                        (goto _label))))
                  (:OnNotifyBegin
                    (switch name _notifyname
                      (:AttackTrace
                        (CallFunction|AttackTrace))))))))
          (:OnFail
            (goto _label_3)))))))

(event Custom|ReleaseAttack
  (bind _charactermovement (Variables|Character|GetCharacterMovement))
  (bind _attributecomponent_enemy (Variables|Default|GetAttributeComponent_ENEMY))
  ;[1 1 1] CHASE PLAYER STATE
  (Utilities|FlowControl|DoOnce false) ; enters at Reset
)

(event Custom|TrackPlayer
  ;[1 1 1] Track Player
  (Variables|Default|GetAttackTarget
    (:then
      (if (Variables|Default|GetIsAiAttackingPlayer)
        (Transformation|SetActorRotation (Math|Rotator|MakeRotator 0.0 0.0 (.yaw (Math|Rotator|FindLookatRotation (Transformation|GetActorLocation) (Transformation|GetActorLocation (Variables|Default|GetAttackTarget))))))
        (Utilities|FlowControl|Delay 0.01)
        (CallFunction|TrackPlayer)))
    (:else)))

(event EventBeginPlay
  (bind _mesh (Variables|Character|GetMesh))
  (bind _returnvalue (Transformation|GetSocketTransform _mesh "SwordSocket" "RTS_Actor"))
  ;[1 1 1] Beginplay
  (Utilities|FlowControl|Sequence
    (:then_0
      (CallFunction|BehaviourUnit)
      (Components|SkinnedMesh|HideBonebyName (Variables|Character|GetMesh) "Hand_R_001" "PBO_None")
      (for _array_element (Variables|Default|GetAi_Items)
        (if (Utilities|Enum|Equal(Enum) _array_element "NewEnumerator2")
          (AddComponent|AddStaticMeshComponent false (Math|Transform|MakeTransform (.location _returnvalue) (.rotation _returnvalue) (.scale _returnvalue))))))
    (:then_1
      (bind _asbp_playercharacter (Utilities|Casting|CastToBP_PLAYERCharacter (Game|GetPlayerCharacter 0)))
      (Variables|Default|SetPlayerRef _asbp_playercharacter))))

(event Game|Damage|EventAnyDamage
  (params (Damage :type Float%20%28single-precision%29) (DamageType :type Damage%20Type%20Object%20Reference) (InstigatedBy :type Controller%20Object%20Reference) (DamageCauser :type Actor%20Object%20Reference))
  (bind _attributecomponent_enemy (Variables|Default|GetAttributeComponent_ENEMY))
  ;[1 1 1] Take Damage
  (bind _output_get (Variables|/Game/Game/Enemy/BaseSkeleton/AttributeComponent_ENEMY.AttributeComponent_ENEMY_C|SetHealth _attributecomponent_enemy (- (Variables|/Game/Game/Enemy/BaseSkeleton/AttributeComponent_ENEMY.AttributeComponent_ENEMY_C|GetHealth _attributecomponent_enemy) Damage)))
  (if (<= _output_get 0.0)
    (Variables|Default|SetIsAiDead true)
    (Variables|Default|SetBehaviourMode "NewEnumerator6")
    (CallFunction|BehaviourUnit)))

(fn ConstructionScript
  (bind _self self)
  (bind _outactors (Actor|GetAllActorsOfClass "/Game/Game/Enemy/BaseSkeleton/EnemyPatrolPoint_BP.EnemyPatrolPoint_BP_C"))
  (Variables|Default|SetPatrolPointRef (Utilities|Array|Get(acopy) _outactors))
  (for _array_element _outactors
    (if (< (Transformation|GetDistanceTo _array_element _self) (Transformation|GetDistanceTo (Variables|Default|GetPatrolPointRef) _self))
      (Variables|Default|SetPatrolPointRef _array_element))))

(fn UpdatePatrolPoint
  (bind _self self)
  (bind _outactors (Actor|GetAllActorsOfClass "/Game/Game/Enemy/BaseSkeleton/EnemyPatrolPoint_BP.EnemyPatrolPoint_BP_C"))
  (for _array_element _outactors
    (if (< (Transformation|GetDistanceTo _array_element _self) (Transformation|GetDistanceTo (Variables|Default|GetPatrolPointRef) _self))
      (Variables|Default|SetPatrolPointRef _array_element))))

(fn AttackTrace
  (bind _returnvalue (Transformation|GetActorLocation))
  (bind _attributecomponent_enemy (Variables|Default|GetAttributeComponent_ENEMY))
  (bind _strength (Variables|/Game/Game/Enemy/BaseSkeleton/AttributeComponent_ENEMY.AttributeComponent_ENEMY_C|GetStrength _attributecomponent_enemy))
  (bind _strengthmodifier (Variables|/Game/Game/Enemy/BaseSkeleton/AttributeComponent_ENEMY.AttributeComponent_ENEMY_C|GetStrengthModifier _attributecomponent_enemy))
  (bind _returnvalue_2 (* _strength 0.2))
  (bind _returnvalue_3 (+ _returnvalue_2 _strengthmodifier))
  (bind (_outhit _returnvalue_4) (Collision|SphereTraceByChannel _returnvalue (+ _returnvalue (* (Transformation|GetActorForwardVector) (Variables|Default|GetAiAttackRange))) (Variables|Default|GetAiAttackRadius) "TraceTypeQuery3" false 0 "ForDuration"))
  (if _returnvalue_4
    (Game|Damage|ApplyDamage (.HitActor (Collision|BreakHitResult _outhit)) (Math|Random|RandomFloatinRange (- _returnvalue_3 (Math|Random|RandomFloatinRange 1.0 6.0)) _returnvalue_3) 0 0)))