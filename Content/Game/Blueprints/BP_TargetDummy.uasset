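; Target dummy actor that shows floating damage numbers when it takes point damage.
; On a hit, it looks up the hit bone in its CombatComponent's BoneDamageModifiers map, defaulting to 1.0 when absent, and scales the damage by that modifier.
; It then spawns a W_DamageNumbers widget with the result, placed at the actor's location plus a small random offset projected to screen space.
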(event Game|Damage|EventPointDamage
  (params (Damage :type Float%20%28single-precision%29) (DamageType :type Damage%20Type%20Object%20Reference) (HitLocation :type Vector :default "0, 0, 0") (HitNormal :type Vector :default "0, 0, 0") (HitComponent :type Primitive%20Component%20Object%20Reference) (BoneName :type Name :default "None") (ShotFromDirection :type Vector :default "0, 0, 0") (InstigatedBy :type Controller%20Object%20Reference) (DamageCauser :type Actor%20Object%20Reference) (HitInfo :type Hit%20Result%20Structure%20%28by%20ref%29))
  (bind _modifier (CallFunction|GetDamageBoneModifier HitInfo))
  (bind _returnvalue (UserInterface|CreateWidget "/Game/Game/UI/W_DamageNumbers.W_DamageNumbers_C" 0 (.ScreenPosition (Class|GameplayStatics|ProjectWorldtoScreen (Game|GetPlayerController 0) (+ (Transformation|GetActorLocation) (* (Math|Random|RandomUnitVector) (Math|Random|RandomFloatinRange 0.0 5e+01))) false)) (* _modifier Damage)))
  (UserInterface|Viewport|AddtoViewport _returnvalue 0))

(fn ConstructionScript)

(fn GetDamageBoneModifier
  (params (Hit :type Hit%20Result%20Structure))
  (bind _hitbonename (Collision|BreakHitResult Hit))
  (bind _combatcomponent (Variables|Default|GetCombatComponent))
  (bind _bonedamagemodifiers (Variables|/Game/Game/Blueprints/CombatComponent.CombatComponent_C|GetBoneDamageModifiers _combatcomponent))
  (bind (_value _returnvalue) (Utilities|Map|Find _bonedamagemodifiers _hitbonename))
  (return (Math|Float|SelectFloat _value 1.0 _returnvalue)))