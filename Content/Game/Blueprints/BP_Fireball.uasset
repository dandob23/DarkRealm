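; BP_Fireball is a player fireball ability that takes cast input directly and deals point damage as a hitscan shot, despite its projectile naming.
; IA_Cast start calls Cast, which checks for positive ammo, then line-traces from the camera along its forward vector with debug drawing.
; Ammo is never decremented here; Uncast (on cancel or completion), Reload and Bounce are unfinished stubs.
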(event Input|EnhancedActionEvents|EnhancedInputActionIA_Cast
  (params (ActionValue :type Boolean) (ElapsedSeconds :type Float%20%28double-precision%29) (TriggeredSeconds :type Float%20%28double-precision%29) (InputAction :type Input%20Action%20Object%20Reference :default "/Game/Game/FirstPerson/Input/Actions/IA_Cast.IA_Cast"))
  (:Started
    (CallFunction|Cast))
  (:Canceled
    (CallFunction|Uncast :!label _label))
  (:Completed
    (goto _label)))

(event EventBeginPlay
  (Input|EnableInput (Game|GetPlayerController 0)))

(fn ConstructionScript)

(fn FireBallProjectile
  (bind _returnvalue (Game|GetPlayerCameraManager 0))
  (bind _returnvalue_2 (Transformation|GetActorLocation _returnvalue))
  (bind (_outhit _returnvalue_3) (Collision|LineTraceByChannel _returnvalue_2 (+ _returnvalue_2 (* (Transformation|GetActorForwardVector _returnvalue) (Variables|Default|GetRange))) "TraceTypeQuery3" false 0 "ForDuration"))
  (if _returnvalue_3
    (Game|Damage|ApplyPointDamage (.HitActor (Collision|BreakHitResult _outhit)) (Variables|Default|GetDamageNormal) (Math|Vector|GetUnitDirection(Vector) (.TraceStart (Collision|BreakHitResult _outhit)) (.TraceEnd (Collision|BreakHitResult _outhit))) _outhit 0 self)))

(fn Cast
  (if (CallFunction|CanCastFire)
    (CallFunction|FireBallProjectile)))

(fn Uncast)

(fn Reload)

(fn CanCastFire
  (return (> (Variables|Default|GetCurrentsAmmo) 0)))

(fn Bounce
  (if (CallFunction|CanCastFire)
    _))