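; Shopkeeper Blueprint that opens and closes a shop screen when interacted with.
; On opening, it looks up each expected inventory enum by name in the item info data table and adds found rows uniquely to its inventory.
; It then creates the shop widget with a reference to itself and enables the cursor with game-and-UI input.
; Interacting again removes the widget and restores game-only input.
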(event Custom|ShowShop
  (bind _returnvalue (Game|GetPlayerController 0))
  (bind _returnvalue_2 (UserInterface|CreateWidget "/Game/Game/UI/Shop_W.Shop_W_C"))
  (Variables|/Game/Game/UI/Shop_W.Shop_W_C|SetShopKeeper _returnvalue_2 self)
  (bind _output_get (Variables|Default|SetShopWidgetRef _returnvalue_2))
  (UserInterface|Viewport|AddtoViewport _output_get 0)
  (Input|SetInputModeGameandUI _returnvalue _output_get "DoNotLock" true false)
  (Variables|/Script/Engine.PlayerController|SetbShowMouseCursor _returnvalue true)
  (Variables|Default|SetIsShopOpen true))

(event EventInteract
  (bind _returnvalue (Game|GetPlayerController 0))
  (bind _inventoryexpected (Variables|Default|GetInventoryExpected))
  (if (Variables|Default|GetIsShopOpen)
    (Widget|RemovefromParent (Variables|Default|GetShopWidgetRef))
    (Input|SetInputModeGameOnly _returnvalue false)
    (Variables|/Script/Engine.PlayerController|SetbShowMouseCursor _returnvalue false)
    (Variables|Default|SetIsShopOpen false)
    (else
      (for _index (range 0 (- (Utilities|Array|Length _inventoryexpected) 1))
        (bind _returnvalue_2 (Utilities|GetDataTableRow "/Game/Game/InteractionSystem/DATATABLE_ItemInfo.DATATABLE_ItemInfo" (Utilities|String|StringToName (Utilities|String|EnumtoString (Utilities|Array|Get(acopy) _inventoryexpected _index))))
          (:then
            (Utilities|Array|AddUnique (Variables|Default|GetInventory) _returnvalue_2))))
      (CallFunction|ShowShop))))

(fn ConstructionScript
  (|CallParentFunction))