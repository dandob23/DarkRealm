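; Base interactable item actor that the player can pick up.
; The construction script fills ItemInfo from the item data table, using the ItemName enum's string as the row name.
; Interact, when IsInteractable is set, passes one item to the player character's PickupItem and optionally destroys the actor.
; DropPhysics turns a given interactable into a destroy-on-pickup physics object that blocks most channels but overlaps or ignores selected ones, including Pawn.
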(event EventInteract
  (if (Variables|Default|GetIsInteractable)
    (bind _asbp_playercharacter (Utilities|Casting|CastToBP_PLAYERCharacter (Game|GetPlayerCharacter 0)))
    (Default|PickupItem _asbp_playercharacter (Variables|Default|GetItemInfo) 1)
    (if (Variables|Default|GetShouldDestroy?)
      (Actor|DestroyActor))))

(fn ConstructionScript
  (bind _returnvalue (Utilities|GetDataTableRow "/Game/Game/InteractionSystem/DATATABLE_ItemInfo.DATATABLE_ItemInfo" (Utilities|String|StringToName (Utilities|String|EnumtoString (Variables|Default|GetItemName))))
    (:then
      (Variables|Default|SetItemInfo _returnvalue))))

(fn DropPhysics
  (params (Interactable :type Base%20Interactable%20BP%20Object%20Reference))
  (bind _item (Variables|BaseInteractable_BP_C|GetItem Interactable))
  (Variables|BaseInteractable_BP_C|SetIsInteractable Interactable true)
  (Variables|BaseInteractable_BP_C|SetShouldDestroy? Interactable true)
  (Physics|SetSimulatePhysics _item true)
  (Physics|SetEnableGravity _item true)
  (Variables|/Script/Engine.PrimitiveComponent|SetCanCharacterStepUpOn _item "ECB_Yes")
  (Collision|SetCollisionEnabled _item "QueryAndPhysics")
  (Collision|SetCollisionResponsetoAllChannels _item "ECR_Block")
  (Collision|SetCollisionResponsetoChannel _item "ECC_Pawn" "ECR_Overlap")
  (Collision|SetCollisionResponsetoChannel _item "ECC_GameTraceChannel3" "ECR_Overlap")
  (Collision|SetCollisionResponsetoChannel _item "ECC_Visibility" "ECR_Overlap")
  (Collision|SetCollisionResponsetoChannel _item "ECC_Camera" "ECR_Overlap")
  (Collision|SetCollisionResponsetoChannel _item "ECC_GameTraceChannel2" "ECR_Ignore"))