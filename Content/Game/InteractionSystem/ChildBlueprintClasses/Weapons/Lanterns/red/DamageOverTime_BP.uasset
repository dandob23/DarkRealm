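; Red lantern weapon area effect that deals damage over time to enemies for ten seconds, then deactivates its particles and destroys its sphere and flame.
; Sphere overlaps add "Enemy"-tagged actors to an array that is never pruned, so enemies leaving the area stay targeted.
; A resettable DoOnce repeats damage each second while active.
; Each hit is randomized below 20% of player MagicDamage, though the graph comment says 30%.
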(event OnComponentBeginOverlap(Sphere)
  (params (OverlappedComponent :type Primitive%20Component%20Object%20Reference) (OtherActor :type Actor%20Object%20Reference) (OtherComp :type Primitive%20Component%20Object%20Reference) (OtherBodyIndex :type Integer) (bFromSweep :type Boolean) (SweepResult :type Hit%20Result%20Structure%20%28by%20ref%29))
  (bind _overlappedactors (Variables|Default|GetOverlappedActors))
  (if (Utilities|IsValid OtherActor)
    (if (Actor|ActorHasTag OtherActor "Enemy")
      (Utilities|Array|Add _overlappedactors OtherActor)
      (CallFunction|ApplyDamageTick _overlappedactors))))

(event Custom|Reset%20Damage
  (Utilities|FlowControl|DoOnce false) ; enters at Reset
)

(event Custom|ApplyDamageTick
  (params (Actor :type Array%20of%20Actor%20Object%20References))
  (Utilities|FlowControl|DoOnce false
    (:Completed
      (CallFunction|DamageOverTime Actor)
      (if (Variables|Default|GetActive)
        (Utilities|FlowControl|Delay 1.0)
        (CallFunction|ResetDamage)
        (CallFunction|ApplyDamageTick (Variables|Default|GetOverlappedActors))))))

(event EventBeginPlay
  (Utilities|FlowControl|Sequence
    (:then_0
      (bind _asbp_playercharacter (Utilities|Casting|CastToBP_PLAYERCharacter (Game|GetPlayerCharacter 0)))
      (Variables|Default|SetPlayerRef _asbp_playercharacter))
    (:then_1
      (Variables|Default|SetActive true)
      (Utilities|FlowControl|Delay 1e+01)
      (Variables|Default|SetActive false)
      (Components|Activation|Deactivate (Variables|Default|GetSphere))
      (Components|DestroyComponent (Variables|Default|GetRedFlame)))))

(fn ConstructionScript)

(fn DamageOverTime
  (params (ActorInput :type Array%20of%20Actor%20Object%20References))
  ;[1 1 1] 30% of the magic damage will be damage over time with a max 10dmg subtraction
  (for _array_element ActorInput
    (LocalVariables|SetDamageOverTimeAmount (* (Variables|/Game/Game/Components/AttributeComponent.AttributeComponent_C|GetMagicDamage (Variables|/Game/Game/FirstPerson/Blueprints/BP_PLAYERCharacter.BP_PLAYERCharacter_C|GetAttributeComponent (Variables|Default|GetPlayerRef))) 0.2))
    (Game|Damage|ApplyDamage _array_element (Math|Random|RandomFloatinRange (- (LocalVariables|GetDamageOverTimeAmount) (Math|Random|RandomFloatinRange 0.0 1e+01)) (LocalVariables|GetDamageOverTimeAmount)) 0 0)
    (Development|PrintString (Utilities|String|ToString(Float) (Math|Random|RandomFloatinRange (- (LocalVariables|GetDamageOverTimeAmount) (Math|Random|RandomFloatinRange 0.0 1e+01)) (LocalVariables|GetDamageOverTimeAmount))) true false "(R=1.000000,G=0.278732,B=0.000000,A=1.000000)"))
  (return))