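; Timed blue-lantern slow zone, shown with snow and blue flame effects, that weakens BaseEnemy_BP actors inside its sphere.
; Begin overlap increments each enemy's slow counter and repeatedly halves strength and walk speed by that count.
; End overlap attempts a clamped doubling reversal, using original values cached from only the first enemy affected.
; After ten seconds it restores overlapping enemies to those values, deactivates effects and destroys the sphere and flame.
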(event OnComponentBeginOverlap(Sphere)
  (params (OverlappedComponent :type Primitive%20Component%20Object%20Reference) (OtherActor :type Actor%20Object%20Reference) (OtherComp :type Primitive%20Component%20Object%20Reference) (OtherBodyIndex :type Integer) (bFromSweep :type Boolean) (SweepResult :type Hit%20Result%20Structure%20%28by%20ref%29))
  (if (not (Actor|ActorHasTag OtherActor "Player"))
    (if (== (Utilities|Array|FindItem (Variables|Default|GetActiveSlowDowns) OtherActor) -1)
      (bind _asbase_enemy_bp (Utilities|Casting|CastToBaseEnemy_BP OtherActor))
      (Variables|/Game/Game/Enemy/BaseSkeleton/BaseEnemy_BP.BaseEnemy_BP_C|SetIsAiNotSlowed _asbase_enemy_bp false)
      (Math|Integer|IncrementInt (Variables|/Game/Game/Enemy/BaseSkeleton/BaseEnemy_BP.BaseEnemy_BP_C|GetAiSlowedCounter _asbase_enemy_bp)
        (:%20%20
          (if (Variables|Default|GetFirstTime)
            (Variables|Default|SetOriginal%20Strength (Variables|/Game/Game/Enemy/BaseSkeleton/AttributeComponent_ENEMY.AttributeComponent_ENEMY_C|GetStrength (Variables|/Game/Game/Enemy/BaseSkeleton/BaseEnemy_BP.BaseEnemy_BP_C|GetAttributeComponent_ENEMY _asbase_enemy_bp)))
            (Variables|Default|SetOriginal%20Speed (Variables|/Script/Engine.CharacterMovementComponent|GetMaxWalkSpeed (Variables|/Script/Engine.Character|GetCharacterMovement _asbase_enemy_bp)))
            (Variables|Default|SetFirstTime false))
          (for _index (range 0 (- (Variables|/Game/Game/Enemy/BaseSkeleton/BaseEnemy_BP.BaseEnemy_BP_C|GetAiSlowedCounter _asbase_enemy_bp) 1))
            (Variables|/Game/Game/Enemy/BaseSkeleton/AttributeComponent_ENEMY.AttributeComponent_ENEMY_C|SetStrength (Variables|/Game/Game/Enemy/BaseSkeleton/BaseEnemy_BP.BaseEnemy_BP_C|GetAttributeComponent_ENEMY _asbase_enemy_bp) (* (Variables|/Game/Game/Enemy/BaseSkeleton/AttributeComponent_ENEMY.AttributeComponent_ENEMY_C|GetStrength (Variables|/Game/Game/Enemy/BaseSkeleton/BaseEnemy_BP.BaseEnemy_BP_C|GetAttributeComponent_ENEMY _asbase_enemy_bp)) 0.5))
            (Variables|/Script/Engine.CharacterMovementComponent|SetMaxWalkSpeed (Variables|/Script/Engine.Character|GetCharacterMovement _asbase_enemy_bp) (* (Variables|/Script/Engine.CharacterMovementComponent|GetMaxWalkSpeed (Variables|/Script/Engine.Character|GetCharacterMovement _asbase_enemy_bp)) 0.5)))
          (Utilities|Array|Add (Variables|Default|GetActiveSlowDowns) OtherActor))))))

(event OnComponentEndOverlap(Sphere)
  (params (OverlappedComponent :type Primitive%20Component%20Object%20Reference) (OtherActor :type Actor%20Object%20Reference) (OtherComp :type Primitive%20Component%20Object%20Reference) (OtherBodyIndex :type Integer))
  (if (not (Actor|ActorHasTag "Player"))
    (if (== (Utilities|Array|FindItem (Variables|Default|GetActiveSlowDowns) 0) -1)
      (bind _asbase_enemy_bp (Utilities|Casting|CastToBaseEnemy_BP OtherActor))
      (Utilities|Array|RemoveItem (Variables|Default|GetActiveSlowDowns) OtherActor)
      (Variables|/Game/Game/Enemy/BaseSkeleton/BaseEnemy_BP.BaseEnemy_BP_C|SetIsAiNotSlowed _asbase_enemy_bp true)
      (Math|Integer|DecrementInt (Variables|/Game/Game/Enemy/BaseSkeleton/BaseEnemy_BP.BaseEnemy_BP_C|GetAiSlowedCounter _asbase_enemy_bp)
        (:%20%20
          (for _index (range 0 (- (Variables|/Game/Game/Enemy/BaseSkeleton/BaseEnemy_BP.BaseEnemy_BP_C|GetAiSlowedCounter _asbase_enemy_bp) 1))
            (Variables|/Game/Game/Enemy/BaseSkeleton/AttributeComponent_ENEMY.AttributeComponent_ENEMY_C|SetStrength (Variables|/Game/Game/Enemy/BaseSkeleton/BaseEnemy_BP.BaseEnemy_BP_C|GetAttributeComponent_ENEMY _asbase_enemy_bp) (Math|Float|Clamp(Float) (* (Variables|/Game/Game/Enemy/BaseSkeleton/AttributeComponent_ENEMY.AttributeComponent_ENEMY_C|GetStrength (Variables|/Game/Game/Enemy/BaseSkeleton/BaseEnemy_BP.BaseEnemy_BP_C|GetAttributeComponent_ENEMY _asbase_enemy_bp)) 2.0) (Variables|/Game/Game/Enemy/BaseSkeleton/AttributeComponent_ENEMY.AttributeComponent_ENEMY_C|GetStrength (Variables|/Game/Game/Enemy/BaseSkeleton/BaseEnemy_BP.BaseEnemy_BP_C|GetAttributeComponent_ENEMY _asbase_enemy_bp)) (Variables|Default|GetOriginal%20Strength)))
            (Variables|/Script/Engine.CharacterMovementComponent|SetMaxWalkSpeed (Variables|/Script/Engine.Character|GetCharacterMovement _asbase_enemy_bp) (Math|Float|Clamp(Float) (* (Variables|/Script/Engine.CharacterMovementComponent|GetMaxWalkSpeed (Variables|/Script/Engine.Character|GetCharacterMovement _asbase_enemy_bp)) 2.0) (Variables|/Script/Engine.CharacterMovementComponent|GetMaxWalkSpeed (Variables|/Script/Engine.Character|GetCharacterMovement _asbase_enemy_bp)) (Variables|Default|GetOriginal%20Speed)))))))))

(event EventBeginPlay
  (Utilities|FlowControl|Delay 1e+01)
  (for _array_element (Collision|GetOverlappingActors (Variables|Default|GetSphere) 0 :!class /Script/Engine.PrimitiveComponent)
    (Utilities|Array|RemoveItem (Variables|Default|GetActiveSlowDowns) _array_element)
    (bind _asbase_enemy_bp (Utilities|Casting|CastToBaseEnemy_BP _array_element))
    (Variables|/Game/Game/Enemy/BaseSkeleton/AttributeComponent_ENEMY.AttributeComponent_ENEMY_C|SetStrength (Variables|/Game/Game/Enemy/BaseSkeleton/BaseEnemy_BP.BaseEnemy_BP_C|GetAttributeComponent_ENEMY _asbase_enemy_bp) (Variables|Default|GetOriginal%20Strength))
    (Variables|/Script/Engine.CharacterMovementComponent|SetMaxWalkSpeed (Variables|/Script/Engine.Character|GetCharacterMovement _asbase_enemy_bp) (Variables|Default|GetOriginal%20Speed)))
  (Components|Activation|Deactivate (Variables|Default|Getsnow))
  (Components|DestroyComponent (Variables|Default|GetSphere)))

(fn ConstructionScript)