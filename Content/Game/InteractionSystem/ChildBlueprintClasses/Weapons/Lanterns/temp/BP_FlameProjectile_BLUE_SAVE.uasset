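; Blue lantern flame projectile that explodes on impact, dealing random area damage scaled by the player's magic attributes to Enemy-tagged actors.
; Each hit sphere-traces for damage; the second doubles radius and damage, destroys the projectile and spawns SlowDown_BP.
; Hitting a physics body also applies an impulse and ends it, but spawns SlowDown_BP without setting DestroyLocation.
; Overlap detonates immediately; the damage loop stops at the first non-enemy.
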(event OnComponentBeginOverlap(CollisionComponent)
  (params (OverlappedComponent :type Primitive%20Component%20Object%20Reference) (OtherActor :type Actor%20Object%20Reference) (OtherComp :type Primitive%20Component%20Object%20Reference) (OtherBodyIndex :type Integer) (bFromSweep :type Boolean) (SweepResult :type Hit%20Result%20Structure%20%28by%20ref%29))
  (bind _collisioncomponent (Variables|MyProjectile|GetCollisionComponent))
  (bind _explosionmesh (Variables|Default|GetExplosionMesh))
  (bind _returnvalue (Transformation|GetWorldLocation _collisioncomponent))
  (bind _returnvalue_2 (Transformation|GetWorldTransform _explosionmesh))
  (if (== (Variables|Default|GetBounceCounter) 1)
    (CallFunction|OnActorHitLantern _returnvalue 2)
    (else
      (CallFunction|OnActorHitLantern _returnvalue)))
  (Effects|SpawnEmitteratLocation "/Game/InfinityBladeEffects/Effects/FX_Monsters/FX_Monster_Gruntling/Bomber/P_FireBombExplosion_BLUE.P_FireBombExplosion_BLUE" (.location _returnvalue_2) (.rotation _returnvalue_2) (* (.scale _returnvalue_2) 0.5))
  (Actor|DestroyActor))

(event EventBeginPlay
  (bind _asbp_playercharacter (Utilities|Casting|CastToBP_PLAYERCharacter (Game|GetPlayerCharacter 0)))
  (Variables|Default|SetPlayerRef _asbp_playercharacter))

(event Collision|EventHit
  (params (MyComp :type Primitive%20Component%20Object%20Reference) (Other :type Actor%20Object%20Reference) (OtherComp :type Primitive%20Component%20Object%20Reference) (bSelfMoved :type Boolean) (HitLocation :type Vector :default "0, 0, 0") (HitNormal :type Vector :default "0, 0, 0") (NormalImpulse :type Vector :default "0, 0, 0") (Hit :type Hit%20Result%20Structure%20%28by%20ref%29))
  (bind _returnvalue (Transformation|GetVelocity))
  (bind _explosionmesh (Variables|Default|GetExplosionMesh))
  (bind _explosionmesh_2 (Variables|Default|GetExplosionMesh))
  (bind _explosionmesh_3 (Variables|Default|GetExplosionMesh))
  (bind _returnvalue_2 (Transformation|GetWorldTransform _explosionmesh_2))
  (bind _returnvalue_3 (* _returnvalue 2e+03))
  (bind _returnvalue_4 (Transformation|GetWorldTransform _explosionmesh))
  (bind _returnvalue_5 (Transformation|GetWorldTransform _explosionmesh_3))
  (bind _output_get (Variables|Default|SetHit%20Location HitLocation))
  (bind _output_get_2 (Variables|Default|SetBounceCounter (+ (Variables|Default|GetBounceCounter) 1)))
  (Effects|SpawnEmitteratLocation "/Game/InfinityBladeEffects/Effects/FX_Monsters/FX_Monster_Gruntling/Bomber/P_FireBombExplosion_BLUE.P_FireBombExplosion_BLUE" (.location _returnvalue_4) (.rotation _returnvalue_4) (* (.scale _returnvalue_4) 0.5))
  (CallFunction|OnActorHitLantern _output_get _output_get_2)
  (if (== (Variables|Default|GetBounceCounter) 2)
    (Effects|SpawnEmitteratLocation "/Game/InfinityBladeEffects/Effects/FX_Monsters/FX_Monster_Gruntling/Bomber/P_FireBombExplosion_BLUE.P_FireBombExplosion_BLUE" (.location _returnvalue_5) (.rotation _returnvalue_5) (.scale _returnvalue_5))
    (Variables|Default|SetDestroyLocation (.location _returnvalue_5))
    (Actor|DestroyActor :!label _label)
    (Game|SpawnActorfromClass "/Game/Game/InteractionSystem/ChildBlueprintClasses/Weapons/Lanterns/blue/SlowDown_BP.SlowDown_BP_C" (Math|Conversions|ToTransform(Vector) (Variables|Default|GetDestroyLocation)) "Undefined" "MultiplyWithRoot" 0 0)
    (elif (Physics|IsSimulatingPhysics OtherComp "None")
      (Physics|AddImpulseatLocation OtherComp _returnvalue_3 (Transformation|GetActorLocation) "None")
      (Effects|SpawnEmitteratLocation "/Game/StarterContent/Particles/P_Explosion_BLUE.P_Explosion_BLUE" _returnvalue_3 (.rotation _returnvalue_2) (.scale _returnvalue_2))
      (goto _label))))

(fn ConstructionScript)

(fn OnActorHitLantern
  (params (HitLocation :type Vector) (BounceCounterInput :type Integer))
  (bind _returnvalue (Math|Random|RandomFloatinRange 1.0 6.0))
  (bind _playerref (Variables|Default|GetPlayerRef))
  (bind _attributecomponent (Variables|/Game/Game/FirstPerson/Blueprints/BP_PLAYERCharacter.BP_PLAYERCharacter_C|GetAttributeComponent _playerref))
  (bind _magicmodifier (Variables|/Game/Game/Components/AttributeComponent.AttributeComponent_C|GetMagicModifier _attributecomponent))
  (bind _magicdamage (Variables|/Game/Game/Components/AttributeComponent.AttributeComponent_C|GetMagicDamage _attributecomponent))
  (bind _returnvalue_2 (* _magicdamage 0.2))
  (bind _returnvalue_3 (+ _returnvalue_2 _magicmodifier))
  (bind _returnvalue_4 (- _returnvalue_3 _returnvalue))
  (bind _returnvalue_5 (Math|Random|RandomFloatinRange _returnvalue_4 _returnvalue_3))
  (bind _returnvalue_6 (* _returnvalue_5 2.0))
  (if (== BounceCounterInput 2)
    (LocalVariables|SetExplosionRadius 2e+02)
    (else
      (LocalVariables|SetExplosionRadius 1e+02)))
  (bind (_outhits _returnvalue_7) (Collision|MultiSphereTraceByChannel HitLocation HitLocation (LocalVariables|GetExplosionRadius) "TraceTypeQuery4" false 0 "None"))
  (if _returnvalue_7
    (for (_array_element _array_index) _outhits
      (if (Utilities|IsValid (.HitActor (Collision|BreakHitResult _array_element)))
        (if (Actor|ActorHasTag (.HitActor (Collision|BreakHitResult _array_element)) "Enemy")
          (if (== BounceCounterInput 2)
            (Game|Damage|ApplyDamage (.HitActor (Collision|BreakHitResult (Utilities|Array|Get(acopy) _outhits _array_index))) _returnvalue_6 0 0)
            (Development|PrintString (Utilities|String|ToString(Float) _returnvalue_6) true false "(R=0.000000,G=0.177542,B=1.000000,A=1.000000)")
            (else
              (Game|Damage|ApplyDamage (.HitActor (Collision|BreakHitResult (Utilities|Array|Get(acopy) _outhits _array_index))) _returnvalue_5 0 0)
              (Development|PrintString (Utilities|String|ToString(Float) _returnvalue_5) true false)))
          (else
            (return)))
        (else
          (return))))
    (return)))