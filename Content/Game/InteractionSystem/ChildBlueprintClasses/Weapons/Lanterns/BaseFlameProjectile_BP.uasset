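; Base lantern flame projectile that bounces and deals area magic damage to enemies.
; Each hit runs a sphere trace explosion, with the second bounce using a larger radius and double damage before destroying the projectile and spawning an after-effect.
; Overlaps explode and destroy it immediately, while a lifespan timer triggers a final blast that destroys it only upon damaging an enemy.
; Randomized damage scales with player magic attributes.
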(event OnComponentBeginOverlap(CollisionComponent)
  (params (OverlappedComponent :type Primitive%20Component%20Object%20Reference) (OtherActor :type Actor%20Object%20Reference) (OtherComp :type Primitive%20Component%20Object%20Reference) (OtherBodyIndex :type Integer) (bFromSweep :type Boolean) (SweepResult :type Hit%20Result%20Structure%20%28by%20ref%29))
  (bind _collisioncomponent (Variables|MyProjectile|GetCollisionComponent))
  (bind _explosionmesh (Variables|Default|GetExplosionMesh))
  (bind _returnvalue (Transformation|GetWorldTransform _explosionmesh))
  (bind _returnvalue_2 (Transformation|GetWorldLocation _collisioncomponent))
  (Development|PrintString "OVERLAP" true true "(R=1.000000,G=0.000000,B=0.000000,A=1.000000)" 5.0)
  (if (== (Variables|Default|GetBounceCounter) 1)
    (CallFunction|OnActorHitLantern _returnvalue_2 2)
    (else
      (CallFunction|OnActorHitLantern _returnvalue_2)))
  (Effects|SpawnEmitteratLocation (Variables|Default|GetBounceFX) (.location _returnvalue) (.rotation _returnvalue) (* (.scale _returnvalue) 0.5))
  (Actor|DestroyActor))

(event Custom|LifespanDestroy
  (Utilities|FlowControl|Delay 2e+01)
  (CallFunction|ExplodeonLifespanReached))

(event EventBeginPlay
  (bind _asbp_playercharacter (Utilities|Casting|CastToBP_PLAYERCharacter (Game|GetPlayerCharacter 0)))
  (Variables|Default|SetPlayerRef _asbp_playercharacter)
  (CallFunction|LifespanDestroy))

(event Collision|EventHit
  (params (MyComp :type Primitive%20Component%20Object%20Reference) (Other :type Actor%20Object%20Reference) (OtherComp :type Primitive%20Component%20Object%20Reference) (bSelfMoved :type Boolean) (HitLocation :type Vector :default "0, 0, 0") (HitNormal :type Vector :default "0, 0, 0") (NormalImpulse :type Vector :default "0, 0, 0") (Hit :type Hit%20Result%20Structure%20%28by%20ref%29))
  (bind _explosionmesh (Variables|Default|GetExplosionMesh))
  (bind _explosionmesh_2 (Variables|Default|GetExplosionMesh))
  (bind _returnvalue (Transformation|GetWorldTransform _explosionmesh))
  (bind _returnvalue_2 (Transformation|GetWorldTransform _explosionmesh_2))
  (Development|PrintString "HIT" true true "(R=1.000000,G=0.000000,B=0.000000,A=1.000000)" 5.0)
  (bind _output_get (Variables|Default|SetHit%20Location HitLocation))
  (bind _result (Math|Integer|IncrementInt (Variables|Default|GetBounceCounter))
    (:%20%20
      (Development|PrintString (Utilities|String|ToString(Integer) _result))
      (Effects|SpawnEmitteratLocation (Variables|Default|GetBounceFX) (.location _returnvalue) (.rotation _returnvalue) (* (.scale _returnvalue) 0.5))
      (CallFunction|OnActorHitLantern _output_get (Variables|Default|GetBounceCounter))
      (if (== (Variables|Default|GetBounceCounter) 2)
        (Effects|SpawnEmitteratLocation (Variables|Default|GetBounceFX) (.location _returnvalue_2) (.rotation _returnvalue_2) (.scale _returnvalue_2))
        (Variables|Default|SetDestroyLocation (.location _returnvalue_2))
        (Actor|DestroyActor)
        (Game|SpawnActorfromClass (Variables|Default|GetAfterFX) (Math|Conversions|ToTransform(Vector) (Variables|Default|GetDestroyLocation)) "Undefined" "MultiplyWithRoot" 0 0)))))

(fn ConstructionScript)

(fn OnActorHitLantern
  (params (HitLocation :type Vector) (BounceCounterInput :type Integer))
  (if (== BounceCounterInput 2)
    (LocalVariables|SetExplosionRadius 2e+02)
    (else
      (LocalVariables|SetExplosionRadius 1e+02)))
  (bind (_outhits _returnvalue) (Collision|MultiSphereTraceByChannel HitLocation HitLocation (LocalVariables|GetExplosionRadius) "TraceTypeQuery4" false 0 "None"))
  (if _returnvalue
    ;[1 1 1] Create an array with actors registered once
    (for _array_element _outhits
      (if (== (Utilities|Array|FindItem (LocalVariables|GetActorsHit) (.HitActor (Collision|BreakHitResult _array_element))) -1)
        (Utilities|Array|Add (LocalVariables|GetActorsHit) (.HitActor (Collision|BreakHitResult _array_element)))))
    ;[1 1 1] Foreach of the registered actors, do damage once
    (for _array_element_2 (LocalVariables|GetActorsHit)
      (if (Utilities|IsValid _array_element_2)
        (if (Actor|ActorHasTag _array_element_2 "Enemy")
          (if (== BounceCounterInput 2)
            (CallFunction|DoDamage _array_element_2 2.0)
            (else
              (CallFunction|DoDamage _array_element_2 1.0))))))))

(fn ExplodeonLifespanReached
  (bind _returnvalue (Transformation|GetActorLocation))
  (bind _explosionmesh (Variables|Default|GetExplosionMesh))
  (bind _returnvalue_2 (Transformation|GetWorldTransform _explosionmesh))
  (Effects|SpawnEmitteratLocation (Variables|Default|GetBounceFX) (.location _returnvalue_2) (.rotation _returnvalue_2) (* (.scale _returnvalue_2) 2.0))
  (bind _outhits (Collision|MultiSphereTraceByChannel _returnvalue _returnvalue 2e+02 "TraceTypeQuery4" false 0 "ForDuration"))
  ;[1 1 1] Create an array with actors registered once
  (for _array_element _outhits
    (if (== (Utilities|Array|FindItem (LocalVariables|GetActorsHit) (.HitActor (Collision|BreakHitResult _array_element))) -1)
      (Utilities|Array|Add (LocalVariables|GetActorsHit) (.HitActor (Collision|BreakHitResult _array_element)))))
  ;[1 1 1] Foreach of the registered actors, do damage once
  (for _array_element_2 (LocalVariables|GetActorsHit)
    (if (Utilities|IsValid _array_element_2)
      (if (Actor|ActorHasTag _array_element_2 "Enemy")
        (CallFunction|DoDamage _array_element_2 1.0)
        (Actor|DestroyActor)))))

(fn DoDamage
  (params (DamagedActor :type Actor%20Object%20Reference) (DamageMultiplier :type Float%20%28double-precision%29))
  (bind _returnvalue (Math|Random|RandomFloatinRange 1.0 6.0))
  (bind _playerref (Variables|Default|GetPlayerRef))
  (bind _attributecomponent (Variables|/Game/Game/FirstPerson/Blueprints/BP_PLAYERCharacter.BP_PLAYERCharacter_C|GetAttributeComponent _playerref))
  (bind _magicmodifier (Variables|/Game/Game/Components/AttributeComponent.AttributeComponent_C|GetMagicModifier _attributecomponent))
  (bind _magicdamage (Variables|/Game/Game/Components/AttributeComponent.AttributeComponent_C|GetMagicDamage _attributecomponent))
  (bind _returnvalue_2 (* _magicdamage 0.2))
  (bind _returnvalue_3 (+ _returnvalue_2 _magicmodifier))
  (bind _returnvalue_4 (- _returnvalue_3 _returnvalue))
  (bind _returnvalue_5 (Math|Random|RandomFloatinRange _returnvalue_4 _returnvalue_3))
  (bind _returnvalue_6 (* _returnvalue_5 DamageMultiplier))
  (Game|Damage|ApplyDamage DamagedActor _returnvalue_6 0 0)
  (Development|PrintString (Utilities|String|ToString(Float) _returnvalue_6) true false "(R=0.000000,G=0.177542,B=1.000000,A=1.000000)"))