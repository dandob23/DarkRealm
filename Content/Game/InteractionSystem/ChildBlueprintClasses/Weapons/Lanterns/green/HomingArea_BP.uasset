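; Green lantern area effect that fires homing projectiles at nearby non-player actors for ten seconds.
; A self-restarting detection loop picks random actors overlapping AreaOfDetection, storing HomingTarget and briefly raising ShootAtTarget.
; A parallel delay-polled loop spawns one HomingProjectile_BP at AreaOfSpawn per firing window, using DoOnce gates instead of Tick.
; On expiry it stops detection, deactivates effects and destroys some components, leaving the actor; BounceToNearbyEnemy is an empty stub.
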(event Custom|DetectEnemies
  (bind _areaofdetection (Variables|Default|GetAreaOfDetection))
  (bind _overlappingactors (Collision|GetOverlappingActors _areaofdetection 0 :!class /Script/Engine.PrimitiveComponent))
  (bind _outitem (Utilities|Array|Random _overlappingactors))
  (if (Variables|Default|GetActive)
    (Utilities|FlowControl|DoOnce false
      (:Completed
        (if (Utilities|IsValid _outitem)
          (if (not (Actor|ActorHasTag _outitem "Player"))
            (Variables|Default|SetHomingTarget _outitem)
            (Variables|Default|SetShootAtTarget true)
            (Utilities|FlowControl|Delay 0.5)
            (Variables|Default|SetShootAtTarget false)
            (CallFunction|ResetDetectEnemies)
            (Utilities|FlowControl|Delay 0.01)
            (CallFunction|DetectEnemies)
            (else
              (CallFunction|ResetDetectEnemies :!label _label)
              (Utilities|FlowControl|Delay 0.01)
              (CallFunction|DetectEnemies)))
          (else
            (goto _label)))))))

(event Custom|ResetDetectEnemies
  (bind _areaofdetection (Variables|Default|GetAreaOfDetection))
  (bind _overlappingactors (Collision|GetOverlappingActors _areaofdetection 0 :!class /Script/Engine.PrimitiveComponent))
  (bind _outitem (Utilities|Array|Random _overlappingactors))
  (Utilities|FlowControl|DoOnce false) ; enters at Reset
)

(event Custom|SpawnHomingProjectile
  (if (Variables|Default|GetShootAtTarget)
    (Utilities|FlowControl|DoOnce false
      (:Completed
        (Game|SpawnActorfromClass "/Game/Game/InteractionSystem/ChildBlueprintClasses/Weapons/Lanterns/green/HomingProjectile_BP.HomingProjectile_BP_C" (Math|Conversions|ToTransform(Vector) (Transformation|GetWorldLocation (Variables|Default|GetAreaOfSpawn))) "Undefined" "MultiplyWithRoot" 0 "/Game/InfinityBladeEffects/Effects/FX_Monsters/FX_Monster_Gruntling/Bomber/P_FireBombExplosion_GREEN.P_FireBombExplosion_GREEN" 0 0)
        (CallFunction|ResetSpawnHomingProjectile)
        (if (Variables|Default|GetShootAtTarget) :!label _label
          (Utilities|FlowControl|Delay 0.2)
          (goto _label)
          (else
            (Utilities|FlowControl|Delay 0.01)
            (CallFunction|SpawnHomingProjectile)))))
    (else
      (Utilities|FlowControl|Delay 0.01)
      (CallFunction|SpawnHomingProjectile))))

(event Custom|ResetSpawnHomingProjectile
  (Utilities|FlowControl|DoOnce false) ; enters at Reset
)

(event EventBeginPlay
  (Variables|Default|SetActive true)
  (CallFunction|DetectEnemies)
  (CallFunction|SpawnHomingProjectile)
  (Utilities|FlowControl|Delay 1e+01)
  (Variables|Default|SetActive false)
  (Components|Activation|Deactivate (Variables|Default|GetFire_circle))
  (Components|DestroyComponent (Variables|Default|GetGreenFlame)))

(fn ConstructionScript)

(fn BouncetoNearbyEnemy
  (if (Variables|Default|GetEnemyInRange)
    _))