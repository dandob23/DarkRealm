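; Homing magic projectile for the green lantern weapon that pops upward with random drift, slows to a hover, then seeks enemies.
; A DetectEnemies overlap records the enemy class, which a once-per-second search uses to home on the nearest tagged actor, exploding when none is found.
; Collision switches on after a delay, and an overlap triggers a sphere trace that applies randomized damage from player magic attributes, spawns an effect and destroys the projectile.
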(event OnComponentBeginOverlap(DetectEnemies)
  (params (OverlappedComponent :type Primitive%20Component%20Object%20Reference) (OtherActor :type Actor%20Object%20Reference) (OtherComp :type Primitive%20Component%20Object%20Reference) (OtherBodyIndex :type Integer) (bFromSweep :type Boolean) (SweepResult :type Hit%20Result%20Structure%20%28by%20ref%29))
  (if (Utilities|IsValid OtherActor)
    (if (not (Actor|ActorHasTag OtherActor "Player"))
      (Variables|Default|SetEnemyClass (Utilities|GetClass OtherActor)))))

(event OnComponentBeginOverlap(CollisionComponent)
  (params (OverlappedComponent :type Primitive%20Component%20Object%20Reference) (OtherActor :type Actor%20Object%20Reference) (OtherComp :type Primitive%20Component%20Object%20Reference) (OtherBodyIndex :type Integer) (bFromSweep :type Boolean) (SweepResult :type Hit%20Result%20Structure%20%28by%20ref%29))
  (bind _location (Collision|BreakHitResult SweepResult))
  (bind _returnvalue (Math|Random|RandomFloatinRange 1.0 6.0))
  (bind _playerref (Variables|Default|GetPlayerRef))
  (bind _explosionmesh (Variables|Default|GetExplosionMesh))
  (bind _returnvalue_2 (Transformation|GetWorldTransform _explosionmesh))
  (bind _attributecomponent (Variables|/Game/Game/FirstPerson/Blueprints/BP_PLAYERCharacter.BP_PLAYERCharacter_C|GetAttributeComponent _playerref))
  (bind _magicmodifier (Variables|/Game/Game/Components/AttributeComponent.AttributeComponent_C|GetMagicModifier _attributecomponent))
  (bind _magicdamage (Variables|/Game/Game/Components/AttributeComponent.AttributeComponent_C|GetMagicDamage _attributecomponent))
  (bind _returnvalue_3 (* _magicdamage 0.2))
  (bind _returnvalue_4 (+ _returnvalue_3 _magicmodifier))
  (bind _returnvalue_5 (- _returnvalue_4 _returnvalue))
  (bind _returnvalue_6 (Math|Random|RandomFloatinRange _returnvalue_5 _returnvalue_4))
  (bind _returnvalue_7 (* _returnvalue_6 2.0))
  (bind (_outhits _returnvalue_8) (Collision|MultiSphereTraceByChannel _location _location 1e+02 "TraceTypeQuery4" false 0 "None"))
  (if _returnvalue_8
    (for _array_element _outhits
      (Utilities|FlowControl|DoOnce false
        (:Completed
          (if (Utilities|IsValid (.HitActor (Collision|BreakHitResult _array_element)))
            (if (Actor|ActorHasTag (.HitActor (Collision|BreakHitResult _array_element)) "Enemy")
              (Game|Damage|ApplyDamage (.HitActor (Collision|BreakHitResult _array_element)) _returnvalue_7 0 0)
              (Development|PrintString (Utilities|String|ToString(Float) _returnvalue_7) true false "(R=0.000000,G=0.177542,B=1.000000,A=1.000000)")
              (Effects|SpawnEmitteratLocation (Variables|Default|GetBounceFX) (.location _returnvalue_2) (.rotation _returnvalue_2) (* (.scale _returnvalue_2) 0.3))
              (Actor|DestroyActor))))))))

(event Custom|GoToTarget
  (bind _projectilemovement (Variables|Default|GetProjectileMovement))
  (bind (_homing_target _notarget) (CallFunction|FindHomingTarget))
  (if _notarget
    (CallFunction|ExplodeonLifespanReached)
    (else
      (Variables|/Script/Engine.ProjectileMovementComponent|SetHomingTargetComponent _projectilemovement _homing_target)
      (Variables|/Script/Engine.ProjectileMovementComponent|SetbIsHomingProjectile _projectilemovement true))))

(event Custom|StartInterpolation
  (bind _projectilemovement (Variables|Default|GetProjectileMovement))
  (Variables|/Script/Engine.MovementComponent|SetVelocity _projectilemovement (Math|Vector|MakeVector 0.0 0.0 (Math|Interpolation|FInterpTo (.z (Transformation|GetVelocity)) 0.0 (Utilities|Time|GetWorldDeltaSeconds) 2.0)))
  (if (Math|Float|NearlyEqual(Float) (.z (Variables|/Script/Engine.MovementComponent|GetVelocity _projectilemovement)) 0.0 2e+01)
    (CallFunction|EndInterpolation)
    (else
      (Utilities|FlowControl|Delay 0.01)
      (CallFunction|StartInterpolation))))

(event Custom|EndInterpolation
  (bind _projectilemovement (Variables|Default|GetProjectileMovement))
  (Variables|/Script/Engine.MovementComponent|SetVelocity _projectilemovement "0, 0, 0")
  (Variables|/Script/Engine.ProjectileMovementComponent|SetProjectileGravityScale _projectilemovement 0.6)
  (CallFunction|GotoTarget :!label _label)
  (Utilities|FlowControl|Delay 1.0)
  (goto _label))

(event EventBeginPlay
  (bind _returnvalue (Math|Random|RandomFloatinRange -75.0 75.0))
  (bind _projectilemovement (Variables|Default|GetProjectileMovement))
  (bind _collisioncomponent (Variables|Default|GetCollisionComponent))
  (|CallParentFunction)
  (Collision|SetCollisionResponsetoAllChannels _collisioncomponent "ECR_Ignore")
  (Variables|/Script/Engine.MovementComponent|SetVelocity _projectilemovement (Math|Vector|MakeVector _returnvalue _returnvalue (Math|Random|RandomFloatinRange 1.5e+02 2e+02)))
  (Variables|/Script/Engine.ProjectileMovementComponent|SetProjectileGravityScale _projectilemovement 0.0)
  (Utilities|FlowControl|Delay 1.0)
  (CallFunction|StartInterpolation)
  (Utilities|FlowControl|Delay 1.0)
  (Collision|SetCollisionResponsetoAllChannels _collisioncomponent "ECR_Overlap")
  (Collision|SetCollisionResponsetoChannel _collisioncomponent "ECC_Pawn" "ECR_Ignore")
  (Collision|SetCollisionResponsetoChannel _collisioncomponent "ECC_GameTraceChannel2" "ECR_Ignore"))

(event Collision|EventActorBeginOverlap
  (params (OtherActor :type Actor%20Object%20Reference))
  (|CallParentFunction OtherActor) ; This node is disabled and will not be called.\nDrag off pins to build functionality.
)

(fn ConstructionScript
  (|CallParentFunction))

(fn FindHomingTarget
  (bind _outactors (Actor|GetAllActorsOfClasswithTag (Variables|Default|GetEnemyClass) "Enemy"))
  (if (Utilities|Array|IsEmpty _outactors)
    _
    (else
      (for _array_element _outactors
        (if (< (Math|Vector|VectorLength (- (Transformation|GetActorLocation _array_element) (Transformation|GetActorLocation))) (Variables|Default|GetClosestDistance))
          (Variables|Default|SetClosestDistance (Math|Vector|VectorLength (- (Transformation|GetActorLocation _array_element) (Transformation|GetActorLocation))))
          (Variables|Default|SetHomingTarget _array_element)))
      (if (Utilities|IsValid (Actor|GetComponentbyClass (Variables|Default|GetHomingTarget) "/Script/Engine.SceneComponent"))
        (return (Actor|GetComponentbyClass (Variables|Default|GetHomingTarget) "/Script/Engine.SceneComponent") false)
        (else
          _))))
  (return 0 true))