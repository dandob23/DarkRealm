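; Green flame lantern weapon in the interaction system that aims and launches a referenced projectile along its forward vector.
; A looping timer raises Power each second without a cap, and Fire scales the projectile's initial speed by it.
; Tick predicts that path with persistent debug drawing, writes it to the Points spline and feeds four sampled points to SplineFXRed as a trajectory effect.
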(event Custom|AddPower
  (Variables|Default|SetPower (+ (Variables|Default|GetPower) 1.0)))

(event Custom|Fire
  (bind _projectileref (Variables|Default|GetProjectileRef))
  (Variables|/Script/Engine.MovementComponent|SetVelocity (Variables|/Game/Game/InteractionSystem/ChildBlueprintClasses/Weapons/Lanterns/BaseFlameProjectile_BP.BaseFlameProjectile_BP_C|GetProjectileMovement _projectileref) (* (* (Transformation|GetActorForwardVector) (Variables|/Script/Engine.ProjectileMovementComponent|GetInitialSpeed (Variables|/Game/Game/InteractionSystem/ChildBlueprintClasses/Weapons/Lanterns/BaseFlameProjectile_BP.BaseFlameProjectile_BP_C|GetProjectileMovement (Variables|Default|GetProjectileRef)))) (Variables|Default|GetPower)))
  (Components|Activation|Activate (Variables|/Game/Game/InteractionSystem/ChildBlueprintClasses/Weapons/Lanterns/BaseFlameProjectile_BP.BaseFlameProjectile_BP_C|GetProjectileMovement _projectileref) false))

(event EventBeginPlay
  (|CallParentFunction)
  (bind _asbp_playercharacter (Utilities|Casting|CastToBP_PLAYERCharacter (Game|GetPlayerCharacter 0)))
  (Variables|Default|SetPlayerRef _asbp_playercharacter)
  (Variables|Default|SetProjectileRef (Variables|Default|GetProjectileRef))
  (Utilities|Time|SetTimerbyEvent (delegate Custom|AddPower) 1.0 true))

(event Collision|EventActorBeginOverlap
  (params (OtherActor :type Actor%20Object%20Reference))
  (|CallParentFunction OtherActor) ; This node is disabled and will not be called.\nDrag off pins to build functionality.
)

(event EventTick
  (params (DeltaSeconds :type Float%20%28single-precision%29))
  (bind _points (Variables|Default|GetPoints))
  (bind _splinefx_red (Variables|Default|GetSplineFX_red))
  (|CallParentFunction DeltaSeconds)
  (bind _outpathpositions (Class|GameplayStatics|BlueprintPredictProjectilePathbyTraceChannel (Transformation|GetActorLocation) (* (* (Transformation|GetActorForwardVector) (Variables|/Script/Engine.ProjectileMovementComponent|GetInitialSpeed (Variables|/Game/Game/InteractionSystem/ChildBlueprintClasses/Weapons/Lanterns/BaseFlameProjectile_BP.BaseFlameProjectile_BP_C|GetProjectileMovement (Variables|Default|GetProjectileRef)))) (Variables|Default|GetPower)) true 16.0 "ECC_WorldStatic" false 0 "Persistent"))
  (Spline|SetSplinePoints _points _outpathpositions "Local" true)
  (Effects|Components|ParticleSystem|SetVectorParameter _splinefx_red "Start" (Spline|GetLocationatSplinePoint _points 0 "Local"))
  (Effects|Components|ParticleSystem|SetVectorParameter _splinefx_red "Start_t" (Spline|GetLocationatSplinePoint _points 2 "Local"))
  (Effects|Components|ParticleSystem|SetVectorParameter _splinefx_red "End_t" (Spline|GetLocationatSplinePoint _points 4 "Local"))
  (Effects|Components|ParticleSystem|SetVectorParameter _splinefx_red "End" (Spline|GetLocationatSplinePoint _points 6 "Local")))

(fn ConstructionScript
  (|CallParentFunction))