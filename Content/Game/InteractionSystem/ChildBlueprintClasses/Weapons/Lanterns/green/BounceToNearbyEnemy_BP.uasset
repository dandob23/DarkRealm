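; Green lantern weapon actor that appears to be an unfinished bounce-to-nearby-enemy effect.
; On BeginPlay it caches the player and runs a looping bounce-check timer for a fixed lifetime, then deactivates its particles and destroys its flame and collision components.
; Overlap with a homing projectile sets an in-range flag, clears the enemy attribute reference and triggers the check.
; BounceToNearbyEnemy only tests that flag, with no bounce logic yet.
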(event OnComponentBeginOverlap(CollisionComponent)
  (params (OverlappedComponent :type Primitive%20Component%20Object%20Reference) (OtherActor :type Actor%20Object%20Reference) (OtherComp :type Primitive%20Component%20Object%20Reference) (OtherBodyIndex :type Integer) (bFromSweep :type Boolean) (SweepResult :type Hit%20Result%20Structure%20%28by%20ref%29))
  (bind _asbp_homing_projectile_bp (Utilities|Casting|CastToBP_HomingProjectile_BP OtherActor))
  (Variables|Default|SetHomingProjectileRef _asbp_homing_projectile_bp)
  (Variables|Default|SetEnemyInRange true)
  ;[1 1 1] Cast to enemy attribute component
  (Variables|Default|SetEnemyAttributeComponent 0)
  (CallFunction|BouncetoNearbyEnemy))

(event Custom|BounceToEnemy
  (CallFunction|BouncetoNearbyEnemy))

(event EventBeginPlay
  (Utilities|FlowControl|Sequence
    (:then_0
      (bind _asbp_playercharacter (Utilities|Casting|CastToBP_PLAYERCharacter (Game|GetPlayerCharacter 0)))
      (Variables|Default|SetPlayerRef _asbp_playercharacter))
    (:then_1
      (bind _returnvalue (Utilities|Time|SetTimerbyEvent (delegate Custom|BounceToEnemy) 0.1 true))
      (Utilities|FlowControl|Delay 11.0)
      (Utilities|Time|ClearandInvalidateTimerbyHandle _returnvalue)
      (Components|Activation|Deactivate (Variables|Default|GetFire_circle))
      (Components|DestroyComponent (Variables|Default|GetGreenFlame)))))

(fn ConstructionScript)

(fn BouncetoNearbyEnemy
  (if (Variables|Default|GetEnemyInRange)
    _))