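; Interactable wooden or stone door that the player can open, close, unlock or break.
; Interact runs the door state logic, with locked doors consuming a Key_BP from the player's inventory.
; Opening and closing step the yaw through 90 degrees using self-calling Delay events rather than a Timeline.
; Each damage hit lowers health unless locked (checked on Tick); at zero, a temporary Geometry Collection replaces the mesh.
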(event Custom|OpenDoorAnimation
  (bind _output_get (Variables|Default|SetOpenDoor_Rotation (- (Variables|Default|GetOpenDoor_Rotation) 3.0)))
  (Transformation|SetActorRotation (Math|Rotator|MakeRotator 0.0 0.0 _output_get))
  (if (<= (Variables|Default|GetOpenDoor_Rotation) (- (Variables|Default|GetOriginalOpenDoorRotation) 9e+01))
    (Variables|Default|SetOpenDoor_Rotation (Variables|Default|GetOriginalOpenDoorRotation))
    (else
      (Utilities|FlowControl|Delay 0.01)
      (CallFunction|OpenDoorAnimation))))

(event Custom|CloseDoorAnimation
  (bind _output_get (Variables|Default|SetCloseDoor_Rotation (+ (Variables|Default|GetCloseDoor_Rotation) 3.0)))
  (Transformation|SetActorRotation (Math|Rotator|MakeRotator 0.0 0.0 _output_get))
  (if (>= (Variables|Default|GetCloseDoor_Rotation) (+ (Variables|Default|GetOriginalCloseDoorRotation) 9e+01))
    (Variables|Default|SetCloseDoor_Rotation (Variables|Default|GetOriginalCloseDoorRotation))
    (else
      (Utilities|FlowControl|Delay 0.01)
      (CallFunction|CloseDoorAnimation))))

(event Custom|OnTakeAnyDamage_Event
  (params (DamagedActor :type Actor%20Object%20Reference) (Damage :type Float%20%28single-precision%29) (DamageType :type Damage%20Type%20Object%20Reference) (InstigatedBy :type Controller%20Object%20Reference) (DamageCauser :type Actor%20Object%20Reference))
  (bind _item (Variables|Default|GetItem))
  (bind _item_2 (Variables|Default|GetItem))
  (bind _returnvalue (Transformation|GetRelativeTransform _item))
  (bind _staticmesh (Variables|/Script/Engine.StaticMeshComponent|GetStaticMesh _item_2))
  (if (Variables|Default|GetCanBeBroken)
    (Math|Integer|DecrementInt (Variables|Default|GetDoorHealth)
      (:%20%20
        (if (<= (Variables|Default|GetDoorHealth) 0)
          (Variables|Default|SetDoorBroke true)
          (if (== _staticmesh "/Game/EasyBuildingSystem/Meshes/Structures/Polygonal/Wood/SM_Polygonal_Wood_Door.SM_Polygonal_Wood_Door")
            (bind _returnvalue_2 (AddComponent|AddGeometryCollectionComponent false _returnvalue))
            (Components|Activation|Activate _returnvalue_2 false)
            (Utilities|FlowControl|Delay 0.1)
            (Components|DestroyComponent (Variables|Default|GetBox))
            (Utilities|FlowControl|Delay 5.0)
            (Components|DestroyComponent _returnvalue_2)
            (elif (== _staticmesh "/Game/EasyBuildingSystem/Meshes/Structures/Polygonal/Stone/SM_Polygonal_Stone_Doors.SM_Polygonal_Stone_Doors")
              (bind _returnvalue_3 (AddComponent|AddGeometryCollectionComponent false _returnvalue))
              (Components|Activation|Activate _returnvalue_3 false)
              (Utilities|FlowControl|Delay 0.1)
              (Components|DestroyComponent (Variables|Default|GetBox))
              (Utilities|FlowControl|Delay 5.0)
              (Components|DestroyComponent _returnvalue_3))))))))

(event EventBeginPlay
  (bind _returnvalue (Transformation|GetActorRotation))
  (bind _returnvalue_2 (Transformation|GetActorRotation))
  (bind _item (Variables|Default|GetItem))
  (bind _returnvalue_3 (- (.yaw _returnvalue_2) 9e+01))
  (EventDispatchers|BindEventtoOnTakeAnyDamage (delegate Custom|OnTakeAnyDamage_Event))
  (Variables|Default|SetOpenDoor_Rotation (.yaw _returnvalue_2))
  (Variables|Default|SetOriginalOpenDoorRotation (.yaw _returnvalue_2))
  (Variables|Default|SetCloseDoor_Rotation _returnvalue_3)
  (Variables|Default|SetOriginalCloseDoorRotation _returnvalue_3)
  (if (Variables|Default|GetIsTheDoorWooden?)
    (Components|StaticMesh|SetStaticMesh _item "/Game/EasyBuildingSystem/Meshes/Structures/Polygonal/Wood/SM_Polygonal_Wood_Door.SM_Polygonal_Wood_Door")
    (else
      (Components|StaticMesh|SetStaticMesh _item "/Game/EasyBuildingSystem/Meshes/Structures/Polygonal/Stone/SM_Polygonal_Stone_Doors.SM_Polygonal_Stone_Doors")))
  (bind _asbp_playercharacter (Utilities|Casting|CastToBP_PLAYERCharacter (Game|GetPlayerCharacter 0)))
  (Variables|Default|SetPlayerRef _asbp_playercharacter)
  (switch Utilities|FlowControl|Switch|SwitchonDoorStates_ENUM (Variables|Default|GetDoorStates)
    (:NewEnumerator0
      (Transformation|SetActorRotation (Transformation|GetActorRotation) :!label _label))
    (:NewEnumerator1
      (Transformation|SetActorRotation (Math|Rotator|MakeRotator (.roll _returnvalue) (.pitch _returnvalue) (- (.yaw _returnvalue) 9e+01))))
    (:NewEnumerator2
      (goto _label))))

(event EventTick
  (params (DeltaSeconds :type Float%20%28single-precision%29))
  (if (Utilities|Enum|Equal(Enum) (Variables|Default|GetDoorStates) "NewEnumerator2")
    (Variables|Default|SetCanBeBroken false)
    (else
      (Variables|Default|SetCanBeBroken true))))

(event EventInteract
  (CallFunction|DoorLogic))

(fn ConstructionScript
  (|CallParentFunction))

(fn KeyCheck
  (for _array_element (Variables|/Game/Game/FirstPerson/Blueprints/BP_PLAYERCharacter.BP_PLAYERCharacter_C|GetInventory (Variables|Default|GetPlayerRef))
    (if (== (.ItemClass (Utilities|Struct|BreakSTRUCT_Item_Info _array_element)) "/Game/Game/InteractionSystem/ChildBlueprintClasses/Other/InteractableObjects/Door/Key_BP.Key_BP_C")
      (Variables|Default|SetCanOpenDoor true)
      (Variables|Default|SetKey _array_element)))
  (return (Variables|Default|GetCanOpenDoor)))

(fn DoorLogic
  (switch Utilities|FlowControl|Switch|SwitchonDoorStates_ENUM (Variables|Default|GetDoorStates)
    (:NewEnumerator0
      (Development|PrintString "Door Opened")
      (CallFunction|OpenDoorAnimation)
      (Variables|Default|SetDoorStates "NewEnumerator1"))
    (:NewEnumerator1
      (Development|PrintString "Door Closed")
      (CallFunction|CloseDoorAnimation)
      (Variables|Default|SetDoorStates "NewEnumerator0"))
    (:NewEnumerator2
      (bind _answer (CallFunction|KeyCheck))
      (if _answer
        (Development|PrintString "Door Opened with key")
        (CallFunction|OpenDoorAnimation)
        (Variables|Default|SetDoorStates "NewEnumerator1")
        (Default|RemoveItem (Variables|Default|GetPlayerRef) (Variables|Default|GetKey) 1)
        (Variables|Default|SetKey "")
        (else
          (Development|PrintString "Need a key to open this door..." true true "(R=1.000000,G=1.000000,B=1.000000,A=1.000000)" 1e+01)
          (Variables|Default|SetDoorStates "NewEnumerator2"))))))