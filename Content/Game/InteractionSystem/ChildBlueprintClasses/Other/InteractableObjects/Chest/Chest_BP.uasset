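; Interactable chest that stores items and toggles open and closed on Interact, showing or removing its Chest_W inventory widget and switching input mode.
; The first opening fills Inventory from the InventoryExpected map, using item data table rows.
; The lid swings through self-calling events that step its roll after short delays, without a Timeline.
; PickupItem and RemoveItem adjust stacks, then refresh whichever widget grid was clicked.
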(event Custom|ShowChest
  (bind _returnvalue (Game|GetPlayerController 0))
  ;[1 1 1] ShowChest Event
  (bind _returnvalue_2 (UserInterface|CreateWidget "/Game/Game/UI/Chest_W.Chest_W_C"))
  (Variables|/Game/Game/FirstPerson/Blueprints/BP_PLAYERCharacter.BP_PLAYERCharacter_C|SetChestWidgetRef (Variables|Default|GetPlayerRef) _returnvalue_2)
  (Variables|/Game/Game/UI/Chest_W.Chest_W_C|SetChestRef _returnvalue_2 self)
  (bind _output_get (Variables|Default|SetChestWidgetRef _returnvalue_2))
  (UserInterface|Viewport|AddtoViewport _output_get 0)
  (Input|SetInputModeGameandUI _returnvalue _output_get "DoNotLock" true false)
  (Variables|/Script/Engine.PlayerController|SetbShowMouseCursor _returnvalue true)
  (Variables|Default|SetIsChestOpen true))

(event Custom|OpenChestAnim
  (bind _chestcover (Variables|Default|GetChestCover))
  (bind _returnvalue (Transformation|GetWorldRotation _chestcover))
  ;[1 1 1] Open/Close animations
  (bind _output_get (Variables|Default|SetOpenChest_Rotation (+ (Variables|Default|GetOpenChest_Rotation) 3.0)))
  (Transformation|SetWorldRotation (Variables|Default|GetChestCover) (Math|Rotator|MakeRotator _output_get (.pitch _returnvalue) (.yaw _returnvalue)) false false)
  (if (>= (Variables|Default|GetOpenChest_Rotation) (+ (Variables|Default|GetOpenChest_Rotation_Original) 7e+01))
    (Variables|Default|SetOpenChest_Rotation (Variables|Default|GetOpenChest_Rotation_Original))
    (else
      (Utilities|FlowControl|Delay 0.01)
      (CallFunction|OpenChestAnim))))

(event Custom|CloseChestAnim
  (bind _chestcover (Variables|Default|GetChestCover))
  (bind _returnvalue (Transformation|GetWorldRotation _chestcover))
  ;[1 1 1] Open/Close animations
  (bind _output_get (Variables|Default|SetCloseChest_Rotation (- (Variables|Default|GetCloseChest_Rotation) 3.0)))
  (Transformation|SetWorldRotation (Variables|Default|GetChestCover) (Math|Rotator|MakeRotator _output_get (.pitch _returnvalue) (.yaw _returnvalue)) false false)
  (if (<= (Variables|Default|GetCloseChest_Rotation) (- (Variables|Default|GetCloseChest_Rotation_Original) 7e+01))
    (Variables|Default|SetCloseChest_Rotation (Variables|Default|GetCloseChest_Rotation_Original))
    (else
      (Utilities|FlowControl|Delay 0.01)
      (CallFunction|CloseChestAnim))))

(event EventBeginPlay
  (bind _chestcover (Variables|Default|GetChestCover))
  (bind _returnvalue (Transformation|GetWorldRotation _chestcover))
  (bind _returnvalue_2 (+ (.roll _returnvalue) 7e+01))
  ;[1 1 1] BeginPlay
  (Variables|Default|SetOpenChest_Rotation (.roll _returnvalue))
  (Variables|Default|SetOpenChest_Rotation_Original (.roll _returnvalue))
  (Variables|Default|SetCloseChest_Rotation _returnvalue_2)
  (Variables|Default|SetCloseChest_Rotation_Original _returnvalue_2))

(event EventInteract
  (bind _returnvalue (Game|GetPlayerController 0))
  (bind _inventoryexpected (Variables|Default|GetInventoryExpected))
  ;[1 1 1] On Interact
  (if (Variables|Default|GetIsChestOpen)
    (CallFunction|CloseChestAnim)
    (Widget|RemovefromParent (Variables|Default|GetChestWidgetRef))
    (Input|SetInputModeGameOnly _returnvalue false)
    (Variables|/Script/Engine.PlayerController|SetbShowMouseCursor _returnvalue false)
    (Variables|Default|SetIsChestOpen false)
    (else
      (CallFunction|OpenChestAnim)
      (Utilities|FlowControl|Sequence
        (:then_0
          (Utilities|FlowControl|DoOnce false
            (:Completed
              (bind _keys (Utilities|Map|Keys _inventoryexpected))
              (bind _values (Utilities|Map|Values _inventoryexpected))
              (for _index (range 0 (- (Utilities|Array|Length _keys) 1))
                (bind _returnvalue_2 (Utilities|GetDataTableRow "/Game/Game/InteractionSystem/DATATABLE_ItemInfo.DATATABLE_ItemInfo" (Utilities|String|StringToName (Utilities|String|EnumtoString (Utilities|Array|Get(acopy) _keys _index))))
                  (:then
                    (Utilities|Array|Add (Variables|Default|GetInventory) (Utilities|Struct|MakeSTRUCT_Item_Info (.ItemClass (Utilities|Struct|BreakSTRUCT_Item_Info _returnvalue_2)) (.ItemName (Utilities|Struct|BreakSTRUCT_Item_Info _returnvalue_2)) (.ItemImage (Utilities|Struct|BreakSTRUCT_Item_Info _returnvalue_2)) (Utilities|Array|Get(acopy) _values _index) (.MaxStack (Utilities|Struct|BreakSTRUCT_Item_Info _returnvalue_2)) (.ItemIndex (Utilities|Struct|BreakSTRUCT_Item_Info _returnvalue_2)) (.ItemType (Utilities|Struct|BreakSTRUCT_Item_Info _returnvalue_2)) (.Potency (Utilities|Struct|BreakSTRUCT_Item_Info _returnvalue_2)) (.Price (Utilities|Struct|BreakSTRUCT_Item_Info _returnvalue_2)) (.SellValue (Utilities|Struct|BreakSTRUCT_Item_Info _returnvalue_2)) (.GearScore (Utilities|Struct|BreakSTRUCT_Item_Info _returnvalue_2)) (.ItemDescription (Utilities|Struct|BreakSTRUCT_Item_Info _returnvalue_2)))))))
              (bind _asbp_playercharacter (Utilities|Casting|CastToBP_PLAYERCharacter (Game|GetPlayerCharacter 0)))
              (Variables|Default|SetPlayerRef _asbp_playercharacter))))
        (:then_1
          (CallFunction|ShowChest))))))

(fn ConstructionScript
  (|CallParentFunction))

(fn RemoveItem
  (params (Item :type STRUCT%20Item%20Info%20Structure) (Amount%20to%20remove :type Integer))
  (bind _inventory (Variables|Default|GetInventory))
  (bind _inventory_2 (Variables|Default|GetInventory))
  (bind _chestwidgetref (Variables|Default|GetChestWidgetRef))
  (bind _chestwidgetref_2 (Variables|Default|GetChestWidgetRef))
  (bind _returnvalue (Utilities|Array|FindItem _inventory Item))
  (bind _output (Utilities|Array|Get(acopy) _inventory _returnvalue))
  (bind (_itemclass _itemname _itemimage _currentstack _maxstack _itemindex _itemtype _potency _price _sellvalue) (Utilities|Struct|BreakSTRUCT_Item_Info _output))
  (if (<= (.CurrentStack (Utilities|Struct|BreakSTRUCT_Item_Info _output)) Amount%20to%20remove)
    (Utilities|Array|RemoveIndex _inventory_2 (Utilities|Array|FindItem _inventory_2 Item))
    (else
      (Utilities|Array|SetArrayElem (Variables|Default|GetInventory) _returnvalue (Utilities|Struct|MakeSTRUCT_Item_Info _itemclass _itemname _itemimage (- _currentstack Amount%20to%20remove) _maxstack _itemindex _itemtype _potency _price _sellvalue))))
  (if (Variables|/Game/Game/UI/Chest_W.Chest_W_C|GetClickedChestIcon _chestwidgetref)
    (Utilities|IsValid _chestwidgetref
      (:Is%20Valid
        (Widget|Panel|ClearChildren (Variables|/Game/Game/UI/Chest_W.Chest_W_C|GetChestInventoryGrid _chestwidgetref))
        (Variables|/Game/Game/UI/Chest_W.Chest_W_C|SetClickedChestIcon _chestwidgetref false)
        (Default|RefreshChest _chestwidgetref)))
    (elif (Variables|/Game/Game/UI/Chest_W.Chest_W_C|GetClickedPlayerInvIcon _chestwidgetref)
      (Utilities|IsValid _chestwidgetref_2
        (:Is%20Valid
          (Widget|Panel|ClearChildren (Variables|/Game/Game/UI/Chest_W.Chest_W_C|GetInventoryGrid _chestwidgetref_2))
          (Variables|/Game/Game/UI/Chest_W.Chest_W_C|SetClickedPlayerInvIcon _chestwidgetref false)
          (Default|RefreshChest _chestwidgetref_2)))
      (else
        (Development|PrintString "Chest_BP Remove item error")))))

(fn PickupItem
  (params (Item :type STRUCT%20Item%20Info%20Structure) (AmountToPickup :type Integer))
  (bind (_itemclass _maxstack) (Utilities|Struct|BreakSTRUCT_Item_Info Item))
  (bind (_itemclass_2 _itemname _itemimage _currentstack _maxstack_2 _itemindex _itemtype _potency _price _sellvalue _gearscore _itemdescription) (Utilities|Struct|BreakSTRUCT_Item_Info Item))
  (bind _inventory (Variables|Default|GetInventory))
  (bind _chestwidgetref (Variables|Default|GetChestWidgetRef))
  (bind _chestwidgetref_2 (Variables|Default|GetChestWidgetRef))
  ;[1 1 1 1 40] Scan for items in inventory, and stacks them together
  (bind (_array_element _array_index) (Utilities|Array|ForEachLoopwithBreak (Variables|Default|GetInventory) :!label _label)
    (:LoopBody
      (if (and (== (.ItemClass (Utilities|Struct|BreakSTRUCT_Item_Info _array_element)) _itemclass) (< (.CurrentStack (Utilities|Struct|BreakSTRUCT_Item_Info _array_element)) _maxstack))
        (Variables|Default|SetItemIndex _array_index)
        (Variables|Default|SetFoundItem _array_element)
        (Variables|Default|SetIsItemFound true)
        (goto _label Break)))
    (:Completed
      (if (Variables|Default|GetIsItemFound)
        ;[1 1 1 1 40] If item is already in inventory
        (Utilities|Array|SetArrayElem (Variables|Default|GetInventory) (Variables|Default|GetItemIndex) (Utilities|Struct|MakeSTRUCT_Item_Info (.ItemClass (Utilities|Struct|BreakSTRUCT_Item_Info (Variables|Default|GetFoundItem))) (.ItemName (Utilities|Struct|BreakSTRUCT_Item_Info (Variables|Default|GetFoundItem))) (.ItemImage (Utilities|Struct|BreakSTRUCT_Item_Info (Variables|Default|GetFoundItem))) (+ (.CurrentStack (Utilities|Struct|BreakSTRUCT_Item_Info (Variables|Default|GetFoundItem))) AmountToPickup) (.MaxStack (Utilities|Struct|BreakSTRUCT_Item_Info (Variables|Default|GetFoundItem))) (.ItemIndex (Utilities|Struct|BreakSTRUCT_Item_Info (Variables|Default|GetFoundItem))) (.ItemType (Utilities|Struct|BreakSTRUCT_Item_Info (Variables|Default|GetFoundItem))) (.Potency (Utilities|Struct|BreakSTRUCT_Item_Info (Variables|Default|GetFoundItem))) (.Price (Utilities|Struct|BreakSTRUCT_Item_Info (Variables|Default|GetFoundItem))) (.SellValue (Utilities|Struct|BreakSTRUCT_Item_Info (Variables|Default|GetFoundItem))) (.GearScore (Utilities|Struct|BreakSTRUCT_Item_Info (Variables|Default|GetFoundItem))) (.ItemDescription (Utilities|Struct|BreakSTRUCT_Item_Info (Variables|Default|GetFoundItem)))))
        (else
          ;[1 1 1 1 40] If Item is not in inventory
          (bind _returnvalue (Utilities|Array|Add _inventory Item))
          (Utilities|Array|SetArrayElem _inventory _returnvalue (Utilities|Struct|MakeSTRUCT_Item_Info _itemclass_2 _itemname _itemimage AmountToPickup _maxstack_2 _returnvalue _itemtype _potency _price _sellvalue _gearscore _itemdescription))))
      (if (Variables|/Game/Game/UI/Chest_W.Chest_W_C|GetClickedChestIcon _chestwidgetref)
        (Utilities|IsValid _chestwidgetref
          (:Is%20Valid
            (Widget|Panel|ClearChildren (Variables|/Game/Game/UI/Chest_W.Chest_W_C|GetChestInventoryGrid _chestwidgetref))
            (Variables|/Game/Game/UI/Chest_W.Chest_W_C|SetClickedChestIcon _chestwidgetref false)
            (Default|RefreshChest _chestwidgetref)))
        (elif (Variables|/Game/Game/UI/Chest_W.Chest_W_C|GetClickedPlayerInvIcon _chestwidgetref)
          (Utilities|IsValid _chestwidgetref_2
            (:Is%20Valid
              (Widget|Panel|ClearChildren (Variables|/Game/Game/UI/Chest_W.Chest_W_C|GetInventoryGrid _chestwidgetref_2))
              (Variables|/Game/Game/UI/Chest_W.Chest_W_C|SetClickedPlayerInvIcon _chestwidgetref false)
              (Default|RefreshChest _chestwidgetref_2)))
          (else
            (Development|PrintString "Chest_BP Remove item error")))))))