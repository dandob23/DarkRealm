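; Interactable item pouch that acts as a small loot container, opening and closing a chest widget on Interact.
; The first interaction builds its inventory from the InventoryExpected map using item data table rows, then caches the player.
; RemoveItem and PickupItem adjust or merge stacks, then refresh the widget grid matching the clicked icon.
; DestroyItemPouch closes the widget, restores game-only input and optionally destroys the actor.
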(event Custom|ShowItemPouch
  (bind _returnvalue (Game|GetPlayerController 0))
  ;[1 1 1] ShowItemPouch Event
  (bind _returnvalue_2 (UserInterface|CreateWidget "/Game/Game/UI/Chest_W.Chest_W_C"))
  (Variables|/Game/Game/FirstPerson/Blueprints/BP_PLAYERCharacter.BP_PLAYERCharacter_C|SetChestWidgetRef (Variables|Default|GetPlayerRef) _returnvalue_2)
  (Variables|/Game/Game/UI/Chest_W.Chest_W_C|SetItemPouchRef _returnvalue_2 self)
  (bind _output_get (Variables|Default|SetItemPouchRef _returnvalue_2))
  (UserInterface|Viewport|AddtoViewport _output_get 0)
  (Input|SetInputModeGameandUI _returnvalue _output_get "DoNotLock" true false)
  (Variables|/Script/Engine.PlayerController|SetbShowMouseCursor _returnvalue true)
  (Variables|Default|SetIsItemPouchOpen true))

(event Custom|DestroyItemPouch
  (params (destroy :type Boolean))
  (bind _returnvalue (Game|GetPlayerController 0))
  ;[1 1 1] On Interact
  (Widget|RemovefromParent (Variables|Default|GetItemPouchRef))
  (Input|SetInputModeGameOnly _returnvalue true)
  (Variables|/Script/Engine.PlayerController|SetbShowMouseCursor _returnvalue false)
  (Variables|Default|SetIsItemPouchOpen false)
  (if destroy
    (Actor|DestroyActor)))

(event EventInteract
  (bind _returnvalue (Game|GetPlayerController 0))
  (bind _inventoryexpected (Variables|Default|GetInventoryExpected))
  ;[1 1 1] On Interact
  (if (Variables|Default|GetIsItemPouchOpen)
    (Widget|RemovefromParent (Variables|Default|GetItemPouchRef))
    (Input|SetInputModeGameOnly _returnvalue true)
    (Variables|/Script/Engine.PlayerController|SetbShowMouseCursor _returnvalue false)
    (Variables|Default|SetIsItemPouchOpen false)
    (if (stale Custom|DestroyItemPouch destroy)
      (Actor|DestroyActor))
    (else
      (Utilities|FlowControl|Sequence
        (:then_0
          (Utilities|FlowControl|DoOnce false
            (:Completed
              (bind _keys (Utilities|Map|Keys _inventoryexpected))
              (bind _values (Utilities|Map|Values _inventoryexpected))
              (for _index (range 0 (- (Utilities|Array|Length _keys) 1))
                (bind _returnvalue_2 (Utilities|GetDataTableRow "/Game/Game/InteractionSystem/DATATABLE_ItemInfo.DATATABLE_ItemInfo" (Utilities|String|StringToName (Utilities|String|EnumtoString (Utilities|Array|Get(acopy) _keys _index))))
                  (:then
                    (Utilities|Array|Add (Variables|Default|GetInventory) (Utilities|Struct|MakeSTRUCT_Item_Info (.ItemClass (Utilities|Struct|BreakSTRUCT_Item_Info _returnvalue_2)) (.ItemName (Utilities|Struct|BreakSTRUCT_Item_Info _returnvalue_2)) (.ItemImage (Utilities|Struct|BreakSTRUCT_Item_Info _returnvalue_2)) (Utilities|Array|Get(acopy) _values _index) (.MaxStack (Utilities|Struct|BreakSTRUCT_Item_Info _returnvalue_2)) (.ItemIndex (Utilities|Struct|BreakSTRUCT_Item_Info _returnvalue_2)) (.ItemType (Utilities|Struct|BreakSTRUCT_Item_Info _returnvalue_2)) (.Potency (Utilities|Struct|BreakSTRUCT_Item_Info _returnvalue_2)) (.Price (Utilities|Struct|BreakSTRUCT_Item_Info _returnvalue_2)) (.SellValue (Utilities|Struct|BreakSTRUCT_Item_Info _returnvalue_2)) (.GearScore (Utilities|Struct|BreakSTRUCT_Item_Info _returnvalue_2)) (.ItemDescription (Utilities|Struct|BreakSTRUCT_Item_Info _returnvalue_2)))))))
              (bind _asbp_playercharacter (Utilities|Casting|CastToBP_PLAYERCharacter (Game|GetPlayerCharacter 0)))
              (Variables|Default|SetPlayerRef _asbp_playercharacter))))
        (:then_1
          (CallFunction|ShowItemPouch))))))

(event EventBeginPlay
  (Variables|Default|SetInventoryExpected (Variables|Default|GetInventoryExpected)))

(fn ConstructionScript
  (|CallParentFunction))

(fn RemoveItem
  (params (item%20info :type STRUCT%20Item%20Info%20Structure) (amount :type Integer))
  (bind _inventory (Variables|Default|GetInventory))
  (bind _inventory_2 (Variables|Default|GetInventory))
  (bind _itempouchref (Variables|Default|GetItemPouchRef))
  (bind _itempouchref_2 (Variables|Default|GetItemPouchRef))
  (bind _returnvalue (Utilities|Array|FindItem _inventory item%20info))
  (bind _output (Utilities|Array|Get(acopy) _inventory _returnvalue))
  (bind (_itemclass _itemname _itemimage _currentstack _maxstack _itemindex _itemtype _potency _price _sellvalue) (Utilities|Struct|BreakSTRUCT_Item_Info _output))
  (if (<= (.CurrentStack (Utilities|Struct|BreakSTRUCT_Item_Info _output)) amount)
    (Utilities|Array|RemoveIndex _inventory_2 (Utilities|Array|FindItem _inventory_2 item%20info))
    (else
      (Utilities|Array|SetArrayElem (Variables|Default|GetInventory) _returnvalue (Utilities|Struct|MakeSTRUCT_Item_Info _itemclass _itemname _itemimage (- _currentstack amount) _maxstack _itemindex _itemtype _potency _price _sellvalue))))
  (if (Variables|/Game/Game/UI/Chest_W.Chest_W_C|GetClickedChestIcon _itempouchref_2)
    (Utilities|IsValid _itempouchref_2
      (:Is%20Valid
        (Widget|Panel|ClearChildren (Variables|/Game/Game/UI/Chest_W.Chest_W_C|GetChestInventoryGrid _itempouchref_2))
        (Variables|/Game/Game/UI/Chest_W.Chest_W_C|SetClickedChestIcon _itempouchref_2 false)
        (Default|RefreshChest _itempouchref_2)))
    (elif (Variables|/Game/Game/UI/Chest_W.Chest_W_C|GetClickedPlayerInvIcon _itempouchref)
      (Utilities|IsValid _itempouchref
        (:Is%20Valid
          (Widget|Panel|ClearChildren (Variables|/Game/Game/UI/Chest_W.Chest_W_C|GetInventoryGrid _itempouchref))
          (Variables|/Game/Game/UI/Chest_W.Chest_W_C|SetClickedPlayerInvIcon _itempouchref false)
          (Default|RefreshChest _itempouchref)))
      (else
        (Development|PrintString "ItemPouch_BP Remove item error")))))

(fn PickupItem
  (params (item%20info :type STRUCT%20Item%20Info%20Structure) (amount :type Integer))
  (bind (_itemclass _maxstack) (Utilities|Struct|BreakSTRUCT_Item_Info item%20info))
  (bind (_itemclass_2 _itemname _itemimage _currentstack _maxstack_2 _itemindex _itemtype _potency _price _sellvalue _gearscore _itemdescription) (Utilities|Struct|BreakSTRUCT_Item_Info item%20info))
  (bind _inventory (Variables|Default|GetInventory))
  (bind _itempouchref (Variables|Default|GetItemPouchRef))
  (bind _itempouchref_2 (Variables|Default|GetItemPouchRef))
  ;[1 1 1 1 40] Scan for items in inventory, and stacks them together
  (bind (_array_element _array_index) (Utilities|Array|ForEachLoopwithBreak (Variables|Default|GetInventory) :!label _label)
    (:LoopBody
      (if (and (== (.ItemClass (Utilities|Struct|BreakSTRUCT_Item_Info _array_element)) _itemclass) (< (.CurrentStack (Utilities|Struct|BreakSTRUCT_Item_Info _array_element)) _maxstack))
        (LocalVariables|SetItemIndex _array_index)
        (LocalVariables|SetFoundItem _array_element)
        (LocalVariables|SetIsItemFound true)
        (goto _label Break)))
    (:Completed
      (if (LocalVariables|GetIsItemFound)
        ;[1 1 1 1 40] If item is already in inventory
        (Utilities|Array|SetArrayElem (Variables|Default|GetInventory) (LocalVariables|GetItemIndex) (Utilities|Struct|MakeSTRUCT_Item_Info (.ItemClass (Utilities|Struct|BreakSTRUCT_Item_Info (LocalVariables|GetFoundItem))) (.ItemName (Utilities|Struct|BreakSTRUCT_Item_Info (LocalVariables|GetFoundItem))) (.ItemImage (Utilities|Struct|BreakSTRUCT_Item_Info (LocalVariables|GetFoundItem))) (+ (.CurrentStack (Utilities|Struct|BreakSTRUCT_Item_Info (LocalVariables|GetFoundItem))) amount) (.MaxStack (Utilities|Struct|BreakSTRUCT_Item_Info (LocalVariables|GetFoundItem))) (.ItemIndex (Utilities|Struct|BreakSTRUCT_Item_Info (LocalVariables|GetFoundItem))) (.ItemType (Utilities|Struct|BreakSTRUCT_Item_Info (LocalVariables|GetFoundItem))) (.Potency (Utilities|Struct|BreakSTRUCT_Item_Info (LocalVariables|GetFoundItem))) (.Price (Utilities|Struct|BreakSTRUCT_Item_Info (LocalVariables|GetFoundItem))) (.SellValue (Utilities|Struct|BreakSTRUCT_Item_Info (LocalVariables|GetFoundItem))) (.GearScore (Utilities|Struct|BreakSTRUCT_Item_Info (LocalVariables|GetFoundItem))) (.ItemDescription (Utilities|Struct|BreakSTRUCT_Item_Info (LocalVariables|GetFoundItem)))))
        (else
          ;[1 1 1 1 40] If Item is not in inventory
          (bind _returnvalue (Utilities|Array|Add _inventory item%20info))
          (Utilities|Array|SetArrayElem _inventory _returnvalue (Utilities|Struct|MakeSTRUCT_Item_Info _itemclass_2 _itemname _itemimage amount _maxstack_2 _returnvalue _itemtype _potency _price _sellvalue _gearscore _itemdescription))))
      (if (Variables|/Game/Game/UI/Chest_W.Chest_W_C|GetClickedChestIcon _itempouchref)
        (Utilities|IsValid _itempouchref
          (:Is%20Valid
            (Widget|Panel|ClearChildren (Variables|/Game/Game/UI/Chest_W.Chest_W_C|GetChestInventoryGrid _itempouchref))
            (Variables|/Game/Game/UI/Chest_W.Chest_W_C|SetClickedChestIcon _itempouchref false)
            (Default|RefreshChest _itempouchref)))
        (elif (Variables|/Game/Game/UI/Chest_W.Chest_W_C|GetClickedPlayerInvIcon _itempouchref)
          (Utilities|IsValid _itempouchref_2
            (:Is%20Valid
              (Widget|Panel|ClearChildren (Variables|/Game/Game/UI/Chest_W.Chest_W_C|GetInventoryGrid _itempouchref_2))
              (Variables|/Game/Game/UI/Chest_W.Chest_W_C|SetClickedPlayerInvIcon _itempouchref false)
              (Default|RefreshChest _itempouchref_2)))
          (else
            (Development|PrintString "ItemPouch_BP Remove item error")))))))